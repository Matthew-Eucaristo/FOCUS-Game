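; Main game mode that runs round start, enemy waves and end-of-round state capture.
; BeginPlay shows a looping-timer countdown with sound cues, which at zero reveals the HUD timer and has every BP_EnemySpawner spawn for CurrentRound.
; SaveRoundLevelandEndit copies turrets, money, weapon ammo and held item into game mode variables, while LoadRoundLevel only prints the round.
; CoinPitchUp raises coin combo pitch, resetting it through a retriggerable delay.
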(event Custom|Coin%20Pitch%20Up
  ;[1 0.8142 0.003424] For Coin Pickup Sound Effects
  (Variables|Default|SetCombo%20Coin%20Pitch (* (Variables|Default|GetCombo%20Coin%20Pitch) 1.05))
  (Utilities|FlowControl|RetriggerableDelay 3.0)
  (Variables|Default|SetCombo%20Coin%20Pitch 1.0))

(event Custom|Countdown
  (bind _count (Variables|Default|GetCount))
  (Math|Integer|DecrementInt _count
    (:%20%20
      (Rendering|Components|TextRender|SetText (Variables|/Game/UI/HUD/WB_Countdown.WB_Countdown_C|GetTextBlock_0 (Variables|Default|GetCountdownWidget)) (Utilities|Text|ToText(Integer) (Variables|Default|GetCount)))
      (switch int _count
        (:0
          (Audio|PlaySound2D "/Game/SoundEffects/Cue_Go.Cue_Go" 1.0 1.0 0.0 0 0)
          (Utilities|Time|InvalidateTimerHandle (stale EventBeginPlay _returnvalue_2))
          (Widget|RemovefromParent (Variables|Default|GetCountdownWidget))
          (CallFunction|SpawnWave)
          (bind _asbp_controllable_character (Utilities|Casting|CastToBP_ControllableCharacter (Game|GetPlayerCharacter 0)))
          (Widget|SetVisibility (Variables|/Game/UI/HUD/WB_PlayerHUD.WB_PlayerHUD_C|GetWB_Timer (Variables|/Game/Characters/BP_ControllableCharacter.BP_ControllableCharacter_C|GetPlayerHUD _asbp_controllable_character)) "Visible"))
        (:1
          (Audio|PlaySound2D "/Game/SoundEffects/Counting/1.1" 1.0 1.0 0.0 0 0))
        (:2
          (Audio|PlaySound2D "/Game/SoundEffects/Counting/2.2" 1.0 1.0 -0.2 0 0))
        (:3
          (Audio|PlaySound2D "/Game/SoundEffects/Counting/3.3" 1.0 1.0 0.0 0 0))
        (:4
          (Audio|PlaySound2D "/Game/SoundEffects/Counting/4.4" 1.0 1.0 0.0 0 0))
        (:5
          (Audio|PlaySound2D "/Game/SoundEffects/Counting/5.5" 1.0 1.0 0.0 0 0))))))

(event Custom|Load%20Round%20Level
  (bind _current_round (Variables|Default|GetCurrent%20Round))
  (if (!= _current_round 1)
    (Development|PrintString (Utilities|String|Append "Current Round : " (Utilities|String|ToString(Integer) _current_round)))))

(event Custom|Save%20Round%20Level%20and%20End%20it
  (bind _asbp_controllable_character (Utilities|Casting|CastToBP_ControllableCharacter (Game|GetPlayerCharacter 0)))
  (bind _output_get (Variables|Default|SetAs%20BP%20Controllable%20Character _asbp_controllable_character))
  (Utilities|FlowControl|Sequence
    (:then_0
      ;[1 1 1] Save the existing turrets
      (Utilities|Array|Clear (Variables|Default|GetTurret%20Transforms))
      (bind _outactors (Actor|GetAllActorsOfClass "/Game/Characters/Turrets/BP_Turrets.BP_Turrets_C"))
      (for _array_element _outactors
        (Utilities|Array|Add (Variables|Default|GetTurret%20Transforms) (Utilities|Struct|MakeFTurretTransformStruct (Utilities|GetClass _array_element) (Transformation|GetActorTransform _array_element)))))
    (:then_1
      ;[1 1 1] Get Money
      (Variables|Default|SetCurrent%20Money (Variables|/Game/Characters/BP_ControllableCharacter.BP_ControllableCharacter_C|GetMoney _output_get)))
    (:then_2
      ;[1 1 1] Saving Weapons
      (bind _outactors_2 (Actor|GetAllActorsOfClass "/Game/Weapons/BP_Weapon_Base.BP_Weapon_Base_C"))
      (for _array_element_2 _outactors_2
        (if (Utilities|Array|ContainsItem (Variables|/Game/Characters/BP_ControllableCharacter.BP_ControllableCharacter_C|GetListWeapon _output_get) (Utilities|GetClass _array_element_2))
          (Utilities|Array|Add (Variables|Default|GetCurrent%20Weapons) (Utilities|Struct|MakeFCurrentWeaponStruct (Utilities|GetClass _array_element_2) (Variables|/Game/Weapons/BP_Weapon_Base.BP_Weapon_Base_C|GetCurrent%20Ammo _array_element_2) (Variables|/Game/Weapons/BP_Weapon_Base.BP_Weapon_Base_C|GetReserve%20Ammo _array_element_2))))))
    (:then_3
      (bind _outactors_3 (Actor|GetAllActorsOfClass "/Game/Item/BP_Item.BP_Item_C"))
      (if (Utilities|Array|ContainsItem _outactors_3 (Variables|/Game/Characters/BP_ControllableCharacter.BP_ControllableCharacter_C|GetItemHeld _output_get))
        (Variables|Default|SetCurrent%20Item%20Held (Variables|/Game/Characters/BP_ControllableCharacter.BP_ControllableCharacter_C|GetItemHeld _output_get))))))

(event EventBeginPlay
  (bind _returnvalue (UserInterface|CreateWidget "/Game/UI/HUD/WB_Countdown.WB_Countdown_C"))
  (bind _output_get (Variables|Default|SetCountdownWidget _returnvalue))
  (UserInterface|Viewport|AddtoViewport _output_get 0)
  (bind _returnvalue_2 (Utilities|Time|SetTimerbyEvent (delegate Custom|Countdown) 1.0 true)))

(fn ConstructionScript)

(fn SpawnWave
  (bind _asgm_game_mode_main (Utilities|Casting|CastToGM_GameModeMain (Game|GetGameMode)))
  (bind _outactors (Actor|GetAllActorsOfClass "/Game/Characters/Enemies/EnemySpawner/BP_EnemySpawner.BP_EnemySpawner_C"))
  (for _array_element _outactors
    (Default|SpawnWave _array_element (Variables|GM_GameModeMain_C|GetCurrent%20Round _asgm_game_mode_main)))
  (Development|PrintString "Wave Spawned, All Spawner Set"))