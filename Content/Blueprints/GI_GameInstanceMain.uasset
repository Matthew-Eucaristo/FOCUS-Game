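; Game instance that carries player and school progress between rounds of a round-based game with weapons, turrets and subject grades.
; Ending a round stores turrets, money, weapons, held item, HUD icons and task scores, then reopens the school level, or computes final grades and opens the final level after the last round.
; Loading restores that state, respawns turrets and assigns subject tasks from a schedule DataTable.
; It also starts music that persists across level transitions.
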(event Custom|Save%20Round%20Level%20and%20End%20It
  (bind _current_weapon_texture (Variables|Default|GetCurrent%20Weapon%20Texture))
  (bind _subject_gradings (Variables|Default|GetSubject%20Gradings))
  (bind _asbp_controllable_character (Utilities|Casting|CastToBP_ControllableCharacter (Game|GetPlayerCharacter 0)))
  (bind _output_get (Variables|Default|SetAs%20BP%20Controllable%20Character _asbp_controllable_character))
  (Utilities|FlowControl|Sequence
    (:then_0
      ;[1 1 1] Save the existing turrets
      (Utilities|Array|Clear (Variables|Default|GetTurret%20Transforms))
      (bind _outactors (Actor|GetAllActorsOfClass "/Game/Characters/Turrets/BP_Turrets.BP_Turrets_C"))
      (for _array_element _outactors
        (if (not (Actor|ActorHasTag _array_element "IGNORE"))
          (Utilities|Array|Add (Variables|Default|GetTurret%20Transforms) (Utilities|Struct|MakeFTurretTransformStruct (Utilities|GetClass _array_element) (Transformation|GetActorTransform _array_element))))))
    (:then_1
      ;[1 1 1] Save Money
      (Variables|Default|SetCurrent%20Money (Variables|/Game/Characters/BP_ControllableCharacter.BP_ControllableCharacter_C|GetMoney _output_get)))
    (:then_2
      ;[1 1 1] Saving Weapons
      (bind _outactors_2 (Actor|GetAllActorsOfClass "/Game/Weapons/BP_Weapon_Base.BP_Weapon_Base_C"))
      (Variables|Default|SetCurrent%20List%20Weapon (Variables|/Game/Characters/BP_ControllableCharacter.BP_ControllableCharacter_C|GetListWeapon _output_get))
      (for _array_element_2 _outactors_2
        (if (Utilities|Array|ContainsItem (Variables|/Game/Characters/BP_ControllableCharacter.BP_ControllableCharacter_C|GetListWeapon _output_get) (Utilities|GetClass _array_element_2))
          (Utilities|Array|Add (Variables|Default|GetCurrent%20Weapons) (Utilities|Struct|MakeFCurrentWeaponStruct (Utilities|GetClass _array_element_2) (Variables|/Game/Weapons/BP_Weapon_Base.BP_Weapon_Base_C|GetCurrent%20Ammo _array_element_2) (Variables|/Game/Weapons/BP_Weapon_Base.BP_Weapon_Base_C|GetReserve%20Ammo _array_element_2))))))
    (:then_3
      ;[1 1 1] Save Items
      (bind _outactors_3 (Actor|GetAllActorsOfClass "/Game/Item/BP_Item.BP_Item_C"))
      (if (== (Utilities|Array|Length _outactors_3) 2)
        (for _array_element_3 _outactors_3
          (if (not (Actor|ActorHasTag _array_element_3 "IGNORE"))
            (Variables|Default|SetCurrent%20Item%20Held (Utilities|Struct|MakeFCurrentItemStruct (Utilities|GetClass (Variables|/Game/Characters/BP_ControllableCharacter.BP_ControllableCharacter_C|GetItemHeld _output_get)) (Variables|/Game/Item/BP_Item.BP_Item_C|GetNumberOwned _array_element_3)))))
        (else
          (Variables|Default|SetCurrent%20Item%20Held (Utilities|Struct|MakeFCurrentItemStruct 0)))))
    (:then_4
      ;[1 1 1] Save Inventory display
      (Utilities|Map|Add _current_weapon_texture 0 (Variables|/Game/UI/HUD/WB_PlayerHUD.WB_PlayerHUD_C|GetT_Weapon1 (Variables|/Game/Characters/BP_ControllableCharacter.BP_ControllableCharacter_C|GetPlayerHUD (Variables|Default|GetAs%20BP%20Controllable%20Character))))
      (Utilities|Map|Add _current_weapon_texture 1 (Variables|/Game/UI/HUD/WB_PlayerHUD.WB_PlayerHUD_C|GetT_Weapon2 (Variables|/Game/Characters/BP_ControllableCharacter.BP_ControllableCharacter_C|GetPlayerHUD (Variables|Default|GetAs%20BP%20Controllable%20Character))))
      (Utilities|Map|Add _current_weapon_texture 2 (Variables|/Game/UI/HUD/WB_PlayerHUD.WB_PlayerHUD_C|GetT_Weapon3 (Variables|/Game/Characters/BP_ControllableCharacter.BP_ControllableCharacter_C|GetPlayerHUD (Variables|Default|GetAs%20BP%20Controllable%20Character)))))
    (:then_5
      ;[1 1 1] Save Subject Task Completion
      (for (_array_element_4 _array_index) (Variables|Default|GetSubjects)
        (Utilities|Array|SetArrayElem _subject_gradings _array_index (+ (Utilities|Array|Get(acopy) _subject_gradings _array_index) (.TaskPercent (Utilities|Struct|BreakFSubjectStruct _array_element_4))))
        (Utilities|Array|SetArrayElem (Variables|Default|GetCurrent%20Round%20Subject%20Gradings) _array_index (.TaskPercent (Utilities|Struct|BreakFSubjectStruct _array_element_4)))))
    (:then_6
      ;[1 1 1] Increment the current round
      (bind _result (Math|Integer|IncrementInt (Variables|Default|GetCurrent%20Round))
        (:%20%20
          ;[1 1 1] Save the equipped weapon
          (Variables|Default|SetCurrent%20Equipped%20Weapon (Utilities|GetClass (Variables|/Game/Characters/BP_ControllableCharacter.BP_ControllableCharacter_C|GetEquippedWeapon _output_get)))
          (if (== _result 11)
            (CallFunction|CalculateFinalScore)
            ;[1 1 1] Open the final level
            (Game|OpenLevel(byObjectReference) "/Game/Maps/School/FinalSchoolLevel.FinalSchoolLevel")
            (else
              ;[1 1 1] Enter the new round
              (Game|OpenLevel(byObjectReference) "/Game/Maps/School/SchoolLevel.SchoolLevel"))))))))

(event Custom|Calculate%20Final%20Score
  (bind _subject_gradings (Variables|Default|GetSubject%20Gradings))
  (bind _subjects (Variables|Default|GetSubjects))
  (for (_array_element _array_index) _subject_gradings
    (Utilities|Array|SetArrayElem _subject_gradings _array_index (/ _array_element 6.0)))
  (for (_ _array_index_2) _subjects
    (Utilities|Array|SetArrayElem _subject_gradings _array_index_2 (/ (+ (.SubjectMasteryPercent (Utilities|Struct|BreakFSubjectStruct (Utilities|Array|Get(acopy) _subjects _array_index_2))) (Utilities|Array|Get(acopy) _subject_gradings _array_index_2)) 2.0))))

(event Custom|Load%20Round%20Level
  (bind _current_item_held (Variables|Default|GetCurrent%20Item%20Held))
  (bind _subjects (Variables|Default|GetSubjects))
  (bind _current_weapon_texture (Variables|Default|GetCurrent%20Weapon%20Texture))
  (bind (_itemclass _itemcount) (Utilities|Struct|BreakFCurrentItemStruct _current_item_held))
  (bind _asbp_controllable_character (Utilities|Casting|CastToBP_ControllableCharacter (Game|GetPlayerCharacter 0)))
  (bind _output_get (Variables|Default|SetAs%20BP%20Controllable%20Character _asbp_controllable_character))
  (Utilities|FlowControl|Sequence
    (:then_0
      ;[1 1 1] Set item in hand
      (if (Utilities|IsValidClass _itemclass)
        (bind _returnvalue (Actor|GetActorOfClass _itemclass))
        (Variables|/Game/Item/BP_Item.BP_Item_C|SetNumberOwned _returnvalue _itemcount)
        (Variables|/Game/Characters/BP_ControllableCharacter.BP_ControllableCharacter_C|SetItemHeld _output_get _returnvalue)
        (else
          (Variables|/Game/Characters/BP_ControllableCharacter.BP_ControllableCharacter_C|SetItemHeld _output_get 0)))
      ;[1 1 1] Set the equipped weapon
      (bind _returnvalue_2 (Actor|GetActorOfClass (Variables|Default|GetCurrent%20Equipped%20Weapon)))
      (Variables|/Game/Characters/BP_ControllableCharacter.BP_ControllableCharacter_C|SetEquippedWeapon _output_get _returnvalue_2))
    (:then_1
      ;[1 1 1] Load Texture inventory yang baru
      (Variables|/Game/UI/HUD/WB_PlayerHUD.WB_PlayerHUD_C|SetT_Weapon1 (Variables|/Game/Characters/BP_ControllableCharacter.BP_ControllableCharacter_C|GetPlayerHUD (Variables|Default|GetAs%20BP%20Controllable%20Character)) (.Value (Utilities|Map|Find _current_weapon_texture 0)))
      (Variables|/Game/UI/HUD/WB_PlayerHUD.WB_PlayerHUD_C|SetT_Weapon2 (Variables|/Game/Characters/BP_ControllableCharacter.BP_ControllableCharacter_C|GetPlayerHUD (Variables|Default|GetAs%20BP%20Controllable%20Character)) (.Value (Utilities|Map|Find _current_weapon_texture 1)))
      (Variables|/Game/UI/HUD/WB_PlayerHUD.WB_PlayerHUD_C|SetT_Weapon3 (Variables|/Game/Characters/BP_ControllableCharacter.BP_ControllableCharacter_C|GetPlayerHUD (Variables|Default|GetAs%20BP%20Controllable%20Character)) (.Value (Utilities|Map|Find _current_weapon_texture 2))))
    (:then_2
      ;[1 1 1] Load the current money
      (Variables|/Game/Characters/BP_ControllableCharacter.BP_ControllableCharacter_C|SetMoney (Variables|Default|GetAs%20BP%20Controllable%20Character) (Variables|Default|GetCurrent%20Money)))
    (:then_3
      ;[1 1 1] Placing Turrets
      (for _array_element (Variables|Default|GetTurret%20Transforms)
        (bind _returnvalue_3 (AI|SpawnAIFromClass (.TurretClass (Utilities|Struct|BreakFTurretTransformStruct _array_element)) 0 (.Location (Math|Transform|BreakTransform (.TurretTransform (Utilities|Struct|BreakFTurretTransformStruct _array_element)))) (.Rotation (Math|Transform|BreakTransform (.TurretTransform (Utilities|Struct|BreakFTurretTransformStruct _array_element)))) true 0))
        (Utilities|FlowControl|DelayUntilNextTick)
        (bind _asbp_turrets (Utilities|Casting|CastToBP_Turrets _returnvalue_3))
        (Variables|/Game/Characters/Turrets/BP_Turrets.BP_Turrets_C|SetbIsPlaced _asbp_turrets true)
        (Variables|/Game/Characters/Turrets/BP_Turrets.BP_Turrets_C|SetTurretState _asbp_turrets "NewEnumerator1")))
    (:then_4
      ;[1 1 1] Set Weapons
      (Variables|/Game/Characters/BP_ControllableCharacter.BP_ControllableCharacter_C|SetListWeapon (Variables|Default|GetAs%20BP%20Controllable%20Character) (Variables|Default|GetCurrent%20List%20Weapon))
      (bind _outactors (Actor|GetAllActorsOfClass "/Game/Weapons/BP_Weapon_Base.BP_Weapon_Base_C"))
      (for _array_element_2 (Variables|Default|GetCurrent%20Weapons)
        (for _array_element_3 _outactors
          (if (== (Utilities|GetClass _array_element_3) (.WeaponClass (Utilities|Struct|BreakFCurrentWeaponStruct _array_element_2)))
            (Variables|/Game/Weapons/BP_Weapon_Base.BP_Weapon_Base_C|SetCurrent%20Ammo _array_element_3 (.CurrentAmmo (Utilities|Struct|BreakFCurrentWeaponStruct _array_element_2)))
            (Variables|/Game/Weapons/BP_Weapon_Base.BP_Weapon_Base_C|SetReserve%20Ammo _array_element_3 (.ReserveAmmo (Utilities|Struct|BreakFCurrentWeaponStruct _array_element_2)))))))
    (:then_5
      ;[1 1 1] Load Subject's Tasks
      (bind _returnvalue_4 (Utilities|GetDataTableRow "/Game/SchoolSystem/DT_SubjectSchedule.DT_SubjectSchedule" (Utilities|String|StringToName (Utilities|String|ToString(Integer) (Variables|Default|GetCurrent%20Round))))
        (:then
          (for (_array_element_4 _array_index) _subjects
            (Utilities|Array|SetArrayElem _subjects _array_index (Utilities|Struct|MakeFSubjectStruct (.SubjectID (Utilities|Struct|BreakFSubjectStruct _array_element_4)) (.SubjectMasteryPercent (Utilities|Struct|BreakFSubjectStruct _array_element_4)) 0.0 false)))
          (for (_array_element_5 _array_index_2) _subjects
            (if (Utilities|Enum|Equal(Enum) (.SubjectID (Utilities|Struct|BreakFSubjectStruct _array_element_5)) (.Subject0StringID (Utilities|Struct|BreakFSubjectScheduleStruct _returnvalue_4)))
              (Utilities|Array|SetArrayElem _subjects _array_index_2 (Utilities|Struct|MakeFSubjectStruct (.SubjectID (Utilities|Struct|BreakFSubjectStruct _array_element_5)) (.SubjectMasteryPercent (Utilities|Struct|BreakFSubjectStruct _array_element_5)) (.TaskPercent (Utilities|Struct|BreakFSubjectStruct _array_element_5)) true))))
          (for (_array_element_6 _array_index_3) _subjects
            (if (Utilities|Enum|Equal(Enum) (.SubjectID (Utilities|Struct|BreakFSubjectStruct _array_element_6)) (.Subject1StringID (Utilities|Struct|BreakFSubjectScheduleStruct _returnvalue_4)))
              (Utilities|Array|SetArrayElem _subjects _array_index_3 (Utilities|Struct|MakeFSubjectStruct (.SubjectID (Utilities|Struct|BreakFSubjectStruct _array_element_6)) (.SubjectMasteryPercent (Utilities|Struct|BreakFSubjectStruct _array_element_6)) (.TaskPercent (Utilities|Struct|BreakFSubjectStruct _array_element_6)) true))))
          (for (_array_element_7 _array_index_4) _subjects
            (if (Utilities|Enum|Equal(Enum) (.SubjectID (Utilities|Struct|BreakFSubjectStruct _array_element_7)) (.Subject2StringID (Utilities|Struct|BreakFSubjectScheduleStruct _returnvalue_4)))
              (Utilities|Array|SetArrayElem _subjects _array_index_4 (Utilities|Struct|MakeFSubjectStruct (.SubjectID (Utilities|Struct|BreakFSubjectStruct _array_element_7)) (.SubjectMasteryPercent (Utilities|Struct|BreakFSubjectStruct _array_element_7)) (.TaskPercent (Utilities|Struct|BreakFSubjectStruct _array_element_7)) true)))))))))

(fn SetforSubjects
  (params (New%20Structure :type F%20Subject%20Struct%20Structure) (Index%20in%20Array :type Integer))
  (bind _subjects (Variables|Default|GetSubjects))
  (Utilities|Array|SetArrayElem _subjects Index%20in%20Array New%20Structure)
  (return (Utilities|Array|Get(acopy) _subjects Index%20in%20Array)))

(fn GetforSubjects
  (params (Index%20in%20Array :type Integer))
  (return (Utilities|Array|Get(acopy) (Variables|Default|GetSubjects) Index%20in%20Array)))

(fn PlayBackgroundMusic
  (params (Sound%20Cue%20to%20play :type Sound%20Cue%20Object%20Reference))
  (bind _returnvalue (Audio|SpawnSound2D Sound%20Cue%20to%20play 1.0 1.0 0.0 0 true))
  (bind _output_get (Variables|Default|SetBackground%20Music%20Audio%20Component _returnvalue))
  (return _output_get))