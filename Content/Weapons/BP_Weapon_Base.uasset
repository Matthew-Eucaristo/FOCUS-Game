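; Base weapon Blueprint that handles fire-rate gating, magazine and reserve ammo, and reloading, with no projectile or damage logic.
; Fire blocks shooting until a timer calls EnableFire, which re-arms it or triggers Reload when empty.
; A DoOnce guards the delayed reload, which plays a sound, shows the player's HUD reload widget and moves reserve ammo.
; EnableFire records camera rotation for ResetRecoil, which is not called here and still prints debug text.
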(event Custom|Enable%20Fire
  (Variables|Default|SetIs%20Firing false)
  (if (and (> (Variables|Default|GetCurrent%20Ammo) 0) (Variables|Default|GetbIsNotReloading))
    (Variables|Default|SetCan%20Shoot true)
    (Utilities|FlowControl|RetriggerableDelay 0.2)
    (bind _asbp_controllable_character (Utilities|Casting|CastToBP_ControllableCharacter (Game|GetPlayerCharacter 0)))
    (Variables|Default|SetStartRotation (Transformation|GetWorldRotation (Variables|/Game/Characters/BP_ControllableCharacter.BP_ControllableCharacter_C|GetFirst%20Person%20Camera _asbp_controllable_character)))
    (else
      (Variables|Default|SetCan%20Shoot false)
      (CallFunction|Reload))))

(event Custom|DecreaseAmmo
  (bind _result (Math|Integer|DecrementInt (Variables|Default|GetCurrent%20Ammo))
    (:%20%20
      (Variables|Default|SetCurrent%20Ammo _result))))

(event Custom|Reset%20Reloading
  (Utilities|FlowControl|DoOnce false) ; enters at Reset
)

(event Custom|Reset%20Recoil
  (bind _returnvalue (Game|GetPlayerCharacter 0))
  (bind _startrotation (Variables|Default|GetStartRotation))
  (bind _asbp_controllable_character (Utilities|Casting|CastToBP_ControllableCharacter (Game|GetPlayerCharacter 0)))
  (if (Utilities|Operators|NotEqual(!=) (Transformation|GetWorldRotation (Variables|/Game/Characters/BP_ControllableCharacter.BP_ControllableCharacter_C|GetFirst%20Person%20Camera _asbp_controllable_character)) (Variables|Default|GetStartRotation) 1e+01)
    (Development|PrintString "Hello")
    (Pawn|Input|AddControllerPitchInput _returnvalue (- (.pitch _startrotation) (.pitch (Transformation|GetWorldRotation (Variables|/Game/Characters/BP_ControllableCharacter.BP_ControllableCharacter_C|GetFirst%20Person%20Camera _asbp_controllable_character)))))
    (Pawn|Input|AddControllerYawInput _returnvalue (- (.yaw _startrotation) (.yaw (Transformation|GetWorldRotation (Variables|/Game/Characters/BP_ControllableCharacter.BP_ControllableCharacter_C|GetFirst%20Person%20Camera _asbp_controllable_character)))))))

(event EventBeginPlay)

(event Collision|EventActorBeginOverlap
  (params (OtherActor :type Actor%20Object%20Reference)))

(event EventStopFire)

(event EventTick
  (params (DeltaSeconds :type Float%20%28single-precision%29)))

(event EventFire
  (if (and (Variables|Default|GetCan%20Shoot) (Variables|Default|GetbIsNotReloading))
    (Utilities|Time|SetTimerbyEvent (delegate Custom|Enable%20Fire) (/ 1.0 (Variables|Default|GetFire%20Rate)))
    (Variables|Default|SetCan%20Shoot false)
    (Variables|Default|SetIs%20Firing true)))

(event EventReload
  (if (and (> (Variables|Default|GetReserve%20Ammo) 1) (< (Variables|Default|GetCurrent%20Ammo) (Variables|Default|GetMagazine%20Capacity)))
    (Utilities|FlowControl|DoOnce false
      (:Completed
        (CallFunction|StopFire)
        (bind _asbp_controllable_character (Utilities|Casting|CastToBP_ControllableCharacter (Game|GetPlayerCharacter 0)))
        (Audio|PlaySound2D "/Game/SoundEffects/war_reloading.war_reloading" 1.0 1.0 0.0 0 0)
        (Variables|/Game/UI/HUD/WB_Reload.WB_Reload_C|SetDeltaTime (Variables|/Game/UI/HUD/WB_PlayerHUD.WB_PlayerHUD_C|GetWB_Reload (Variables|/Game/Characters/BP_ControllableCharacter.BP_ControllableCharacter_C|GetPlayerHUD _asbp_controllable_character)) 0.0)
        (Widget|SetVisibility (Variables|/Game/UI/HUD/WB_PlayerHUD.WB_PlayerHUD_C|GetWB_Reload (Variables|/Game/Characters/BP_ControllableCharacter.BP_ControllableCharacter_C|GetPlayerHUD _asbp_controllable_character)) "Visible")
        (Variables|Default|SetCan%20Shoot false)
        (Variables|Default|SetbIsNotReloading false)
        (Utilities|FlowControl|Delay (Variables|Default|GetReload%20Duration))
        (bind _output_get (Variables|Default|SetTemp%20Ammo (Variables|Default|GetCurrent%20Ammo)))
        (Variables|Default|SetCurrent%20Ammo (Math|Integer|Min(Integer) (Variables|Default|GetMagazine%20Capacity) (Variables|Default|GetReserve%20Ammo)))
        (Variables|Default|SetReserve%20Ammo (- (Variables|Default|GetReserve%20Ammo) (- (Math|Integer|Min(Integer) (Variables|Default|GetMagazine%20Capacity) (Variables|Default|GetReserve%20Ammo)) _output_get)))
        (Variables|Default|SetCan%20Shoot true)
        (Variables|Default|SetbIsNotReloading true)
        (Widget|SetVisibility (Variables|/Game/UI/HUD/WB_PlayerHUD.WB_PlayerHUD_C|GetWB_Reload (Variables|/Game/Characters/BP_ControllableCharacter.BP_ControllableCharacter_C|GetPlayerHUD _asbp_controllable_character)) "Hidden")
        (CallFunction|ResetReloading)))
    (else
      (Development|PrintString "I need more bullets"))))

(fn ConstructionScript)