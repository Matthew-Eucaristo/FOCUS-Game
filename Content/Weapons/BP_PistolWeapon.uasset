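; Pistol weapon Blueprint that extends a parent weapon class with hitscan firing and pistol-specific sounds.
; Fire line-traces on Visibility from the player character's first-person camera, applies damage to the hit actor and decreases ammo.
; It then adds random pitch and yaw recoil and spawns a Niagara bullet trail at the character's spawn point.
; Reload and switch events call the parent, then play their sound cues.
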(event EventBeginPlay
  (|CallParentFunction) ; This node is disabled and will not be called.\nDrag off pins to build functionality.
)

(event EventFire
  (bind _returnvalue (Game|GetPlayerCharacter 0))
  (|CallParentFunction)
  (bind _asbp_controllable_character (Utilities|Casting|CastToBP_ControllableCharacter (Game|GetPlayerCharacter 0)))
  (bind _outhit (Collision|LineTraceByChannel (Transformation|GetWorldLocation (Variables|/Game/Characters/BP_ControllableCharacter.BP_ControllableCharacter_C|GetFirst%20Person%20Camera _asbp_controllable_character)) (+ (Transformation|GetWorldLocation (Variables|/Game/Characters/BP_ControllableCharacter.BP_ControllableCharacter_C|GetFirst%20Person%20Camera _asbp_controllable_character)) (* (Math|Vector|GetForwardVector (Variables|/Game/Characters/BP_ControllableCharacter.BP_ControllableCharacter_C|GetFirst%20Person%20Camera _asbp_controllable_character)) (Variables|Default|GetShootDistance))) "TraceTypeQuery1" false 0 "None"))
  (Audio|PlaySound2D "/Game/Weapons/SFX/Cue_PistolShoot.Cue_PistolShoot" 1.0 1.0 0.0 0 0)
  ;[0.4015 0.686 1] Apply Damage to the Damageable Object
  (Game|Damage|ApplyDamage (.HitActor (Collision|BreakHitResult _outhit)) (Variables|Default|GetDamage) 0 self)
  (CallFunction|DecreaseAmmo)
  (Utilities|Casting|CastToBP_ControllableCharacter _returnvalue)
  ;[1 1 1] Recoil
  (Pawn|Input|AddControllerPitchInput _returnvalue (Math|Random|RandomFloatinRange -0.2 -0.5))
  (Pawn|Input|AddControllerYawInput _returnvalue (Math|Random|RandomFloatinRange -0.2 0.2))
  (Niagara|SpawnSystematLocation "/Game/Weapons/VFX/NS_bulletTrails.NS_bulletTrails" (.location (Transformation|GetWorldTransform (Variables|/Game/Characters/BP_ControllableCharacter.BP_ControllableCharacter_C|GetNiagara%20Spawn%20Location _asbp_controllable_character))) (.rotation (Transformation|GetWorldTransform (Variables|/Game/Characters/BP_ControllableCharacter.BP_ControllableCharacter_C|GetNiagara%20Spawn%20Location _asbp_controllable_character))) (.scale (Transformation|GetWorldTransform (Variables|/Game/Characters/BP_ControllableCharacter.BP_ControllableCharacter_C|GetNiagara%20Spawn%20Location _asbp_controllable_character)))) ; Spawn Niagara VFX
)

(event EventTick
  (params (DeltaSeconds :type Float%20%28single-precision%29))
  (|CallParentFunction DeltaSeconds))

(event EventReload
  (|CallParentFunction)
  (Audio|PlaySound2D "/Game/Weapons/SFX/Cue_PistolReload.Cue_PistolReload" 1.0 1.0 2.0 0 0))

(event EventSwitchtoThis
  (|CallParentFunction)
  (Audio|PlaySound2D "/Game/Weapons/SFX/Cue_PistolSwitch.Cue_PistolSwitch" 1.0 1.0 0.0 0 0))

(fn ConstructionScript
  (|CallParentFunction))