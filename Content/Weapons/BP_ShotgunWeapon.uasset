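; Shotgun weapon that assigns itself as the equipped weapon of any BP_ControllableCharacter overlapping it.
; Fire calls the parent, then runs ten randomly spread line traces from the player camera, applying damage to each hit actor and drawing debug lines.
; It then plays a laser sound at the world origin, adds random pitch and yaw recoil to player 0's character, and decreases ammo.
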(event EventBeginPlay
  (|CallParentFunction) ; This node is disabled and will not be called.\nDrag off pins to build functionality.
)

(event EventFire
  (bind _returnvalue (Game|GetPlayerCharacter 0))
  (bind _returnvalue_2 (Game|GetPlayerCameraManager 0))
  (bind _spread (Variables|Default|GetSpread))
  (bind _spread_2 (Variables|Default|GetSpread))
  (bind _spread_3 (Variables|Default|GetSpread))
  (bind _transformcomponent (Variables|/Script/Engine.PlayerCameraManager|GetTransformComponent _returnvalue_2))
  (bind _returnvalue_3 (Transformation|GetWorldLocation _transformcomponent))
  (|CallParentFunction)
  (for _index (range 1 10)
    (bind _outhit (Collision|LineTraceByChannel _returnvalue_3 (+ _returnvalue_3 (* (Math|Vector|GetForwardVector _transformcomponent) (Variables|Default|GetShootDistance)) (Math|Vector|MakeVector (Math|Random|RandomFloatinRange (* _spread_2 -1.0) _spread_2) (Math|Random|RandomFloatinRange (* _spread_3 -1.0) _spread_3) (Math|Random|RandomFloatinRange (* _spread -1.0) _spread))) "TraceTypeQuery1" false 0 "ForDuration"))
    ;[0.4015 0.686 1] Apply Damage to the Damageable Object
    (Game|Damage|ApplyDamage (.HitActor (Collision|BreakHitResult _outhit)) (Variables|Default|GetDamage) 0 self))
  (Audio|PlaySoundatLocation "/Game/SoundEffects/laserSmall_004.laserSmall_004" "0, 0, 0" "0, 0, 0" 1.0 1.0 0.0 0 0 0 0) ; Sound for shooting
  (Pawn|Input|AddControllerPitchInput _returnvalue (Math|Random|RandomFloatinRange -2.0 -3.0))
  (Pawn|Input|AddControllerYawInput _returnvalue (Math|Random|RandomFloatinRange -0.2 -0.5))
  (CallFunction|DecreaseAmmo))

(event EventTick
  (params (DeltaSeconds :type Float%20%28single-precision%29))
  (|CallParentFunction DeltaSeconds) ; This node is disabled and will not be called.\nDrag off pins to build functionality.
)

(event Collision|EventActorBeginOverlap
  (params (OtherActor :type Actor%20Object%20Reference))
  (bind _asbp_controllable_character (Utilities|Casting|CastToBP_ControllableCharacter OtherActor))
  (Variables|/Game/Characters/BP_ControllableCharacter.BP_ControllableCharacter_C|SetEquippedWeapon _asbp_controllable_character self))

(fn ConstructionScript
  (|CallParentFunction))