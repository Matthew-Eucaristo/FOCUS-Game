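; BP_MachineGunWeapon is a full-auto hitscan weapon that becomes a BP_ControllableCharacter's equipped weapon on overlap.
; Fire starts a looping timer at FireRate shots per second, cleared by StopFire or empty ammo.
; Each shot line-traces from the player's first-person camera with debug drawing, adds random recoil to controller input, plays a sound at world origin, applies damage and decrements ammo.
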(event Custom|FullAutoFire
  (bind _returnvalue (Game|GetPlayerCharacter 0))
  (if (> (Variables|Default|GetCurrent%20Ammo) 0)
    (bind _outhit (Collision|LineTraceByChannel (Transformation|GetWorldLocation (Variables|/Game/Characters/BP_ControllableCharacter.BP_ControllableCharacter_C|GetFirst%20Person%20Camera (stale EventFire _asbp_controllable_character))) (+ (Transformation|GetWorldLocation (Variables|/Game/Characters/BP_ControllableCharacter.BP_ControllableCharacter_C|GetFirst%20Person%20Camera (stale EventFire _asbp_controllable_character))) (* (Math|Vector|GetForwardVector (Variables|/Game/Characters/BP_ControllableCharacter.BP_ControllableCharacter_C|GetFirst%20Person%20Camera (stale EventFire _asbp_controllable_character))) (Variables|Default|GetShootDistance))) "TraceTypeQuery1" false 0 "ForDuration"))
    (Utilities|Casting|CastToBP_ControllableCharacter _returnvalue)
    (Pawn|Input|AddControllerPitchInput _returnvalue (Math|Random|RandomFloatinRange -0.5 -1.0))
    (Pawn|Input|AddControllerYawInput _returnvalue (Math|Random|RandomFloatinRange -0.5 0.5))
    (Audio|PlaySoundatLocation "/Game/SoundEffects/laserSmall_004.laserSmall_004" "0, 0, 0" "0, 0, 0" 1.0 1.0 0.0 0 0 0 0) ; Sound for shooting
    ;[0.4015 0.686 1] Apply Damage to the Damageable Object
    (Game|Damage|ApplyDamage (.HitActor (Collision|BreakHitResult _outhit)) (Variables|Default|GetDamage) 0 self)
    (CallFunction|DecreaseAmmo)
    (else
      (Utilities|Time|ClearandInvalidateTimerbyHandle (stale EventFire _returnvalue)))))

(event EventBeginPlay
  (|CallParentFunction) ; This node is disabled and will not be called.\nDrag off pins to build functionality.
)

(event EventFire
  (|CallParentFunction)
  (bind _asbp_controllable_character (Utilities|Casting|CastToBP_ControllableCharacter (Game|GetPlayerCharacter 0)))
  (bind _returnvalue (Utilities|Time|SetTimerbyEvent (delegate Custom|FullAutoFire) (/ 1.0 (Variables|Default|GetFire%20Rate)) true)))

(event EventTick
  (params (DeltaSeconds :type Float%20%28single-precision%29))
  (|CallParentFunction DeltaSeconds) ; This node is disabled and will not be called.\nDrag off pins to build functionality.
)

(event Collision|EventActorBeginOverlap
  (params (OtherActor :type Actor%20Object%20Reference))
  (bind _self self)
  (bind _asbp_controllable_character (Utilities|Casting|CastToBP_ControllableCharacter OtherActor))
  (Variables|/Game/Characters/BP_ControllableCharacter.BP_ControllableCharacter_C|SetEquippedWeapon _asbp_controllable_character _self)
  (Development|PrintString (Utilities|GetDisplayName _self)))

(event EventStopFire
  (|CallParentFunction)
  (Utilities|Time|ClearandInvalidateTimerbyHandle (stale EventFire _returnvalue)))

(fn ConstructionScript
  (|CallParentFunction))