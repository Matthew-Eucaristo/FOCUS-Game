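; BP_Store is a store actor that opens a toy box and shows its widget when the player's controllable character comes near.
; Entering the CollisionOpenBox volume reveals the widget, plays the OpenToyBox sequence and enables query-only collision on the widget.
; Leaving hides the widget, plays CloseToyBox and disables its collision, which also starts disabled at BeginPlay.
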(event OnComponentBeginOverlap(CollisionOpenBox)
  (params (OverlappedComponent :type Primitive%20Component%20Object%20Reference) (OtherActor :type Actor%20Object%20Reference) (OtherComp :type Primitive%20Component%20Object%20Reference) (OtherBodyIndex :type Integer) (bFromSweep :type Boolean) (SweepResult :type Hit%20Result%20Structure%20%28by%20ref%29))
  (Utilities|Casting|CastToBP_ControllableCharacter OtherActor)
  (Rendering|SetVisibility (Variables|Default|GetWidget) true false)
  (Class|ActorSequenceComponent|PlaySequence (Variables|Default|GetOpenToyBox))
  (Collision|SetCollisionEnabled (Variables|Default|GetWidget) "QueryOnly"))

(event OnComponentEndOverlap(CollisionOpenBox)
  (params (OverlappedComponent :type Primitive%20Component%20Object%20Reference) (OtherActor :type Actor%20Object%20Reference) (OtherComp :type Primitive%20Component%20Object%20Reference) (OtherBodyIndex :type Integer))
  (Utilities|Casting|CastToBP_ControllableCharacter OtherActor)
  (Rendering|SetVisibility (Variables|Default|GetWidget) false false)
  (Class|ActorSequenceComponent|PlaySequence (Variables|Default|GetCloseToyBox))
  (Collision|SetCollisionEnabled (Variables|Default|GetWidget) "NoCollision"))

(event EventBeginPlay
  (Collision|SetCollisionEnabled (Variables|Default|GetWidget) "NoCollision"))

(event Collision|EventActorBeginOverlap
  (params (OtherActor :type Actor%20Object%20Reference)))

(event EventTick
  (params (DeltaSeconds :type Float%20%28single-precision%29)))

(fn ConstructionScript)