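; Skeleton enemy that chases the player and plays a death animation when killed.
; Every tick, a latent MoveComponentTo drives its capsule toward the player's mesh location over one second, without AI navigation, turning it to the player's rotation with yaw flipped 180 degrees.
; The Dies event plays the death animation once and sets a short lifespan so the actor removes itself.
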(event EventBeginPlay)

(event Collision|EventActorBeginOverlap
  (params (OtherActor :type Actor%20Object%20Reference)))

(event EventTick
  (params (DeltaSeconds :type Float%20%28single-precision%29))
  (bind _returnvalue (Game|GetPlayerCharacter 0))
  (bind _capsulecomponent (Variables|/Script/Engine.Character|GetCapsuleComponent _returnvalue))
  (bind _returnvalue_2 (Transformation|GetWorldRotation _capsulecomponent))
  (bind (_roll _pitch _yaw) (Math|Rotator|BreakRotator _returnvalue_2))
  ;[1 1 1] Logic to chase player
  (Components|MoveComponentTo (Variables|Default|GetCapsuleComponent) (Transformation|GetWorldLocation (Variables|/Script/Engine.Character|GetMesh _returnvalue)) (Math|Rotator|MakeRotator _roll _pitch (- _yaw 1.8e+02)) false false 1.0 false))

(event EventDies
  (Components|Animation|PlayAnimation (Variables|Character|GetMesh) "/Game/Characters/Skeleton/Skeleton_Anim_EnemyArmature_EnemyArmature_EnemyArmature_Death.Skeleton_Anim_EnemyArmature_EnemyArmature_EnemyArmature_Death" false)
  (Actor|SetLifeSpan 2.0))

(fn ConstructionScript)