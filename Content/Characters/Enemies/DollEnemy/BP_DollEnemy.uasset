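; BP_DollEnemy is a doll enemy Blueprint that supplies state-based animations on top of its parent class.
; It overrides PlayAnimationBySTATE, calls the parent, then switches on the state to play idle, walk, run, punch or death clips directly on the mesh.
; Every clip loops, including death.
; Its event graph and construction script add no logic of their own.
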(event EventBeginPlay
  (|CallParentFunction) ; This node is disabled and will not be called.\nDrag off pins to build functionality.
)

(event Collision|EventActorBeginOverlap
  (params (OtherActor :type Actor%20Object%20Reference))
  (|CallParentFunction OtherActor) ; This node is disabled and will not be called.\nDrag off pins to build functionality.
)

(event EventTick
  (params (DeltaSeconds :type Float%20%28single-precision%29))
  (|CallParentFunction DeltaSeconds) ; This node is disabled and will not be called.\nDrag off pins to build functionality.
)

(fn ConstructionScript
  (|CallParentFunction))

(fn PlayAnimationbySTATE
  (params (Current%20STATE :type ENUM_ENEMY_STATE%20Enum :default "NewEnumerator0"))
  (bind _mesh (Variables|Character|GetMesh))
  (|CallParentFunction Current%20STATE)
  (switch Utilities|FlowControl|Switch|SwitchonENUM_ENEMY_STATE Current%20STATE
    (:NewEnumerator0
      (Components|Animation|PlayAnimation _mesh "/Game/Characters/Enemies/DollEnemy/Character_Anim_CharacterArmature_Idle.Character_Anim_CharacterArmature_Idle" true))
    (:NewEnumerator4
      (Components|Animation|PlayAnimation _mesh "/Game/Characters/Enemies/DollEnemy/Character_Anim_CharacterArmature_Walk.Character_Anim_CharacterArmature_Walk" true))
    (:NewEnumerator1
      (Components|Animation|PlayAnimation _mesh "/Game/Characters/Enemies/DollEnemy/Character_Anim_CharacterArmature_Run.Character_Anim_CharacterArmature_Run" true))
    (:NewEnumerator2
      (Components|Animation|PlayAnimation _mesh "/Game/Characters/Enemies/DollEnemy/Character_Anim_CharacterArmature_Punch.Character_Anim_CharacterArmature_Punch" true))
    (:NewEnumerator3
      (Components|Animation|PlayAnimation _mesh "/Game/Characters/Enemies/DollEnemy/Character_Anim_CharacterArmature_Death.Character_Anim_CharacterArmature_Death" true))))