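; BP_PhoneEnemy is a phone enemy that extends a parent enemy class with its own hit sound and destruction effect.
; Getting hit plays a clap cue.
; On death it plays a destroyed cue, adds a geometry collection, hides and disables collision on the mesh and cloud, and triggers a spawned FS_MasterField for Chaos-style fracture.
; The parent's death logic runs after a delay, leaving time for the debris.
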(event EventBeginPlay
  (|CallParentFunction))

(event Collision|EventActorBeginOverlap
  (params (OtherActor :type Actor%20Object%20Reference))
  (|CallParentFunction OtherActor) ; This node is disabled and will not be called.\nDrag off pins to build functionality.
)

(event EventTick
  (params (DeltaSeconds :type Float%20%28single-precision%29))
  (|CallParentFunction DeltaSeconds))

(event EventGotHitSoundEffect
  (Audio|PlaySoundatLocation "/Game/SoundEffects/Cue_Clap.Cue_Clap" (Transformation|GetActorLocation) "0, 0, 0" 1.0 1.0 0.0 0 0 0 0))

(event EventDies
  (bind _staticmesh (Variables|Default|GetStaticMesh))
  (bind _cloud (Variables|Default|GetCloud))
  (Audio|PlaySoundatLocation "/Game/SoundEffects/Cue_PhoneDestroyed.Cue_PhoneDestroyed" (Transformation|GetActorLocation) "0, 0, 0" 1.0 1.0 0.0 0 0 0 0)
  (AddComponent|AddGeometryCollectionComponent false)
  (Rendering|SetVisibility _staticmesh false false)
  (Collision|SetCollisionEnabled _staticmesh "NoCollision")
  (Rendering|SetVisibility _cloud false false)
  (Collision|SetCollisionEnabled _cloud "NoCollision")
  (bind _returnvalue (Game|SpawnActorfromClass "/Engine/EditorResources/FieldNodes/FS_MasterField.FS_MasterField_C" (Transformation|GetActorTransform) "Undefined" "MultiplyWithRoot" 0 0))
  (Variables|/Engine/EditorResources/FieldNodes/FS_MasterField.FS_MasterField_C|SetActivationType _returnvalue "NewEnumerator4")
  (Default|CETrigger _returnvalue)
  (Utilities|FlowControl|Delay 5.0)
  (|CallParentFunction))

(fn ConstructionScript
  (|CallParentFunction))