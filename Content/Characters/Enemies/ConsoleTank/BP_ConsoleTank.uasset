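; Console Tank enemy whose destructible shield absorbs projectile damage, while all other damage goes straight to the parent's damage handling.
; Projectile hits drain ShieldHealth; at depletion a timeline fades the shield's dynamic material opacity, then destroys the component, letting later projectiles through.
; Overlaps on BlockRange play a glass impact sound while the shield is up, with further sounds for getting hit and dying.
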(event OnComponentBeginOverlap(BlockRange)
  (params (OverlappedComponent :type Primitive%20Component%20Object%20Reference) (OtherActor :type Actor%20Object%20Reference) (OtherComp :type Primitive%20Component%20Object%20Reference) (OtherBodyIndex :type Integer) (bFromSweep :type Boolean) (SweepResult :type Hit%20Result%20Structure%20%28by%20ref%29))
  (if (not (Variables|Default|Getis%20Shield%20Destroyed))
    (CallFunction|PlaySFX)))

(event Custom|Damage%20Shield
  (params (Danage :type Float%20%28double-precision%29))
  (if (<= (- (Variables|Default|GetShield%20Health) Danage) 0.0)
    (CallFunction|DestroyShield)
    (else
      (Variables|Default|SetShield%20Health (- (Variables|Default|GetShield%20Health) Danage)))))

(event Custom|Destroy%20Shield
  (Variables|Default|Setis%20Shield%20Destroyed true)
  (bind _opacity (Timeline|Fade%20Away PlayFromStart)
    (:Update
      (Rendering|Material|SetScalarParameterValue (Variables|Default|GetShield%20Material%20Instance) "Opacity" _opacity :!class /Script/Engine.MaterialInstanceDynamic))
    (:Finished
      (Components|DestroyComponent (Variables|Default|GetShield)))))

(event Custom|Play%20SFX
  (Audio|PlaySoundatLocation "/Game/SoundEffects/Cue_GlassImpact.Cue_GlassImpact" (Transformation|GetWorldLocation (Variables|Default|GetCapsuleComponent)) "0, 0, 0" 1.0 1.0 0.0 0 0 0 0))

(event EventBeginPlay
  (|CallParentFunction)
  (bind _returnvalue (Rendering|Material|CreateDynamicMaterialInstance (Variables|Default|GetShield) 0 "/Game/Characters/Enemies/ConsoleTank/Shield/M_ShieldMat.M_ShieldMat" "None" :!class /Script/Engine.PrimitiveComponent))
  (bind _output_get (Variables|Default|SetShield%20Material%20Instance _returnvalue))
  (Rendering|Material|SetScalarParameterValue _output_get "Opacity" 1.0 :!class /Script/Engine.MaterialInstanceDynamic))

(event Collision|EventActorBeginOverlap
  (params (OtherActor :type Actor%20Object%20Reference))
  (|CallParentFunction OtherActor) ; This node is disabled and will not be called.\nDrag off pins to build functionality.
)

(event EventTick
  (params (DeltaSeconds :type Float%20%28single-precision%29))
  (|CallParentFunction DeltaSeconds))

(event EventGotHitSoundEffect
  (Audio|PlaySoundatLocation "/Game/SoundEffects/Cue_GlassCrack.Cue_GlassCrack" (Transformation|GetWorldLocation (Variables|Default|GetCapsuleComponent)) "0, 0, 0" 1.0 1.0 0.0 0 0 0 0))

(event Game|Damage|EventAnyDamage
  (params (Damage :type Float%20%28single-precision%29) (DamageType :type Damage%20Type%20Object%20Reference) (InstigatedBy :type Controller%20Object%20Reference) (DamageCauser :type Actor%20Object%20Reference))
  (if (Actor|ActorHasTag DamageCauser "Projectile")
    (if (Variables|Default|Getis%20Shield%20Destroyed)
      (|CallParentFunction Damage DamageType InstigatedBy DamageCauser :!label _label)
      (else
        (CallFunction|DamageShield Damage)))
    (else
      (goto _label))))

(event EventDies
  (Audio|PlaySoundatLocation "/Game/SoundEffects/Cue_ComputerGlitchAndDies.Cue_ComputerGlitchAndDies" (Transformation|GetActorLocation) "0, 0, 0" 1.0 1.0 0.0 0 0 0 0)
  (|CallParentFunction))

(fn ConstructionScript
  (|CallParentFunction))