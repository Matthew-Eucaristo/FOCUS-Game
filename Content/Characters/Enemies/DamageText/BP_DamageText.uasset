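; BP_DamageText is a short-lived floating damage text actor for enemies.
; On BeginPlay it passes its damage amount and causer to the W_DamageText widget in its widget component.
; It picks a random start point around its spawn location, and a timeline lerps it along a fixed upward diagonal offset before the actor destroys itself.
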(event EventBeginPlay
  (bind _asw_damage_text (Utilities|Casting|CastToW_DamageText (UserInterface|GetWidget (Variables|Default|GetWidget))))
  (Variables|/Game/UI/DamageText/W_DamageText.W_DamageText_C|SetDamageAmount _asw_damage_text (Variables|Default|GetDamage%20Amount))
  (Variables|/Game/UI/DamageText/W_DamageText.W_DamageText_C|SetDamage%20Causer _asw_damage_text (Variables|Default|GetDamage%20Causer))
  (bind _output_get (Variables|Default|SetStart%20Loc (+ (Transformation|GetActorLocation) (* (Math|Vector|SelectVector (* (Math|Random|RandomUnitVector) -1.0) (Math|Random|RandomUnitVector) (Math|Random|RandomBool)) 6e+01))))
  (Variables|Default|SetEnd%20Loc (+ _output_get "-25.000000,-25.000000,50.000000"))
  (bind _move_track (Timeline|Move%20T Play)
    (:Update
      (Transformation|SetActorLocation (Math|Vector|Lerp(Vector) (Variables|Default|GetStart%20Loc) (Variables|Default|GetEnd%20Loc) _move_track) false false))
    (:Finished
      (Actor|DestroyActor))))

(fn ConstructionScript)