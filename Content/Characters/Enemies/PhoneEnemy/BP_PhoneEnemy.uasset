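; Phone enemy that chases the first player character.
; Every Tick it calls MoveComponentTo on its capsule toward the player mesh's world location over one second, rotated by FindLookAtRotation to face it.
; The chase moves the component directly, with no AI or navigation calls.
; BeginPlay and overlap events are disabled stubs, and a TakeDamage call is left unconnected.
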(event EventBeginPlay
  (|CallParentFunction) ; This node is disabled and will not be called.\nDrag off pins to build functionality.
)

(event Collision|EventActorBeginOverlap
  (params (OtherActor :type Actor%20Object%20Reference))
  (|CallParentFunction OtherActor) ; This node is disabled and will not be called.\nDrag off pins to build functionality.
)

(event EventTick
  (params (DeltaSeconds :type Float%20%28single-precision%29))
  (bind _returnvalue (Game|GetPlayerCharacter 0))
  (bind _capsulecomponent (Variables|Default|GetCapsuleComponent))
  (bind _mesh (Variables|/Script/Engine.Character|GetMesh _returnvalue))
  (bind _returnvalue_2 (Transformation|GetWorldLocation _mesh))
  (|CallParentFunction DeltaSeconds)
  ;[1 1 1] Logic to chase player
  (Components|MoveComponentTo _capsulecomponent _returnvalue_2 (Math|Rotator|FindLookatRotation (Transformation|GetWorldLocation _capsulecomponent) _returnvalue_2) false false 1.0 false))

(fn ConstructionScript
  (|CallParentFunction))