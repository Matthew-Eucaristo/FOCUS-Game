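; BP_EnemySpawner spawns AI enemies on a repeating timer, with the type mix and pace set by the current round.
; SpawnWave reads the round's row in DT_RoundWaveSpawnRate to set the type thresholds and start the looping SpawnEnemy timer.
; SpawnEnemy checks a cap on live BP_Enemy actors, then picks one of six classes by comparing a random roll against cumulative thresholds, placing it via GetRandomLocation.
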(event Custom|SpawnEnemy
  ;[1 1 1] Set max enemy spawned
  (bind _outactors (Actor|GetAllActorsOfClass "/Game/Characters/Enemies/BP_Enemy.BP_Enemy_C"))
  (if (<= (Utilities|Array|Length _outactors) 50)
    (Variables|Default|SetRandomFloat (Math|Random|RandomFloatinRange 0.0 1e+02))
    (if (< (Variables|Default|GetRandomFloat) (Utilities|Array|Get(acopy) (Variables|Default|GetEnemyTypeSpawnRate)))
      (AI|SpawnAIFromClass (Utilities|Array|Get(acopy) (Variables|Default|GetEnemiesToSpawn)) 0 (Utilities|GetRandomLocation) "0, 0, 0" true 0)
      (elif (and (>= (Variables|Default|GetRandomFloat) (Utilities|Array|Get(acopy) (Variables|Default|GetEnemyTypeSpawnRate))) (< (Variables|Default|GetRandomFloat) (Utilities|Array|Get(acopy) (Variables|Default|GetEnemyTypeSpawnRate) 1)))
        (AI|SpawnAIFromClass (Utilities|Array|Get(acopy) (Variables|Default|GetEnemiesToSpawn) 1) 0 (Utilities|GetRandomLocation) "0, 0, 0" true 0)
        (elif (and (>= (Variables|Default|GetRandomFloat) (Utilities|Array|Get(acopy) (Variables|Default|GetEnemyTypeSpawnRate) 1)) (< (Variables|Default|GetRandomFloat) (Utilities|Array|Get(acopy) (Variables|Default|GetEnemyTypeSpawnRate) 2)))
          (AI|SpawnAIFromClass (Utilities|Array|Get(acopy) (Variables|Default|GetEnemiesToSpawn) 2) 0 (Utilities|GetRandomLocation) "0, 0, 0" true 0)
          (elif (and (>= (Variables|Default|GetRandomFloat) (Utilities|Array|Get(acopy) (Variables|Default|GetEnemyTypeSpawnRate) 2)) (< (Variables|Default|GetRandomFloat) (Utilities|Array|Get(acopy) (Variables|Default|GetEnemyTypeSpawnRate) 3)))
            (AI|SpawnAIFromClass (Utilities|Array|Get(acopy) (Variables|Default|GetEnemiesToSpawn) 3) 0 (Utilities|GetRandomLocation) "0, 0, 0" true 0)
            (elif (and (>= (Variables|Default|GetRandomFloat) (Utilities|Array|Get(acopy) (Variables|Default|GetEnemyTypeSpawnRate) 3)) (< (Variables|Default|GetRandomFloat) (Utilities|Array|Get(acopy) (Variables|Default|GetEnemyTypeSpawnRate) 4)))
              (AI|SpawnAIFromClass (Utilities|Array|Get(acopy) (Variables|Default|GetEnemiesToSpawn) 4) 0 (Utilities|GetRandomLocation) "0, 0, 0" true 0)
              (elif (>= (Variables|Default|GetRandomFloat) (Utilities|Array|Get(acopy) (Variables|Default|GetEnemyTypeSpawnRate) 4))
                (AI|SpawnAIFromClass (Utilities|Array|Get(acopy) (Variables|Default|GetEnemiesToSpawn) 5) 0 (Utilities|GetRandomLocation) "0, 0, 0" true 0)))))))
    (else
      (Development|PrintString "Max Enemy Reached"))))

(event Custom|Spawn%20Wave
  (params (Current%20Round :type Integer))
  (bind _returnvalue (Utilities|GetDataTableRow "/Game/Characters/Enemies/EnemySpawner/DT_RoundWaveSpawnRate.DT_RoundWaveSpawnRate" (Utilities|String|StringToName (Utilities|String|ToString(Integer) Current%20Round)))
    (:then
      (Variables|Default|SetEnemyTypeSpawnRate (.EnemyTypeSpawnRate (Utilities|Struct|BreakFWaveStucture _returnvalue)))
      (Utilities|Time|SetTimerbyEvent (delegate Custom|SpawnEnemy) (/ 1.0 (.SpawnperSecond (Utilities|Struct|BreakFWaveStucture _returnvalue))) true))
    (:RowNotFound
      (Development|PrintString "ERROR, Row for spawn rate not found!"))))

(event EventBeginPlay)

(fn ConstructionScript)