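; Base enemy character that hunts the player, attacks turrets and controllable characters, and despawns shortly after death.
; A Tick-driven state machine runs idle, searching, targeting, attacking and death, starting searching after a random delay.
; Searching crouch-chases the player, pawn sensing locks tagged targets until lost, and attack-range overlap starts delay-paced damage.
; Children override animation and attack functions, with melee as the default.
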(event OnComponentBeginOverlap(AttackRange)
  (params (OverlappedComponent :type Primitive%20Component%20Object%20Reference) (OtherActor :type Actor%20Object%20Reference) (OtherComp :type Primitive%20Component%20Object%20Reference) (OtherBodyIndex :type Integer) (bFromSweep :type Boolean) (SweepResult :type Hit%20Result%20Structure%20%28by%20ref%29))
  ;[1 0.1832 0.003043] Enemy's Set to Attack Logic
  (if (Actor|ActorHasTag OtherActor "Enemy Target")
    (Utilities|FlowControl|DoOnce false
      (:Completed
        (CallFunction|SetSTATEandAnimation "NewEnumerator2")))))

(event OnSeePawn(PawnSensing)
  (params (Pawn :type Pawn%20Object%20Reference))
  ;[0.5833 0.631 1] On See Pawn Logic
  (if (Actor|ActorHasTag Pawn "Enemy Target")
    (Variables|Default|SetLocked%20Target%20Pawn Pawn)
    (CallFunction|SetSTATEandAnimation "NewEnumerator1")
    ;;[1 1 1] DEBUG: For printing who locked who
    (Development|PrintString (Utilities|String|Append (Utilities|GetDisplayName self) (Utilities|String|MakeLiteralString " has locked ") (Utilities|GetDisplayName Pawn)))))

(event Custom|STATE%20Behaviour
  ;[0.5117 0.7258 1] STATES
  ;;[0.4233 0.8385 1] STATE Behaviour on Tick (Override the STATE Custom Events)
  (switch Utilities|FlowControl|Switch|SwitchonENUM_ENEMY_STATE (Variables|Default|GetSTATE)
    (:NewEnumerator0
      (CallFunction|STATEIDLEBehaviour))
    (:NewEnumerator4
      (CallFunction|STATESEARCHINGBehaviour))
    (:NewEnumerator1
      (CallFunction|STATETargetingBehaviour))
    (:NewEnumerator2
      (CallFunction|STATEATTACKINGBehaviour))
    (:NewEnumerator3
      (CallFunction|STATEDEATHBehaviour))))

(event Custom|Reset%20Attacking%20"Do%20Once"%20after%20no%20enemy%20nearby
  ;[1 0.1832 0.003043] Enemy's Set to Attack Logic
  (Utilities|FlowControl|DoOnce false) ; enters at Reset
)

(event Custom|STATE%20Targeting%20Behaviour
  (bind _self self)
  ;[0.5117 0.7258 1] STATES
  ;;[1 0.8386 0.4106] General Behaviour for TARGETING STATE
  (Character|UnCrouch)
  (if (Utilities|IsValid (Variables|Default|GetLocked%20Target%20Pawn))
    (AI|Navigation|MovetoActor (AI|GetAIController _self) (Variables|Default|GetLocked%20Target%20Pawn) 2.0 true true true 0)
    ;;;[1 1 1] Lose target if too far
    (if (> (Math|Vector|Distance(Vector) (Transformation|GetActorLocation _self) (Transformation|GetActorLocation (Variables|Default|GetLocked%20Target%20Pawn))) (Variables|Default|GetTarget%20Missing%20Treshold))
      (Components|Movement|StopMovementImmediately (Variables|Character|GetCharacterMovement))
      (Variables|Default|SetLocked%20Target%20Pawn 0)
      (CallFunction|SetSTATEandAnimation "NewEnumerator4"))
    (else
      ;;;[1 1 1] Condition if the locked target dies
      (CallFunction|SetSTATEandAnimation "NewEnumerator4") ; If no Locked Target set, change to SEARCHING
      (Variables|Default|SetLocked%20Target%20Pawn 0) ; and empty the target
    )))

(event Custom|STATE%20IDLE%20Behaviour
  ;[0.5117 0.7258 1] STATES
)

(event Custom|STATE%20SEARCHING%20Behaviour
  ;[0.5117 0.7258 1] STATES
  ;;[0.714 0.5477 1] Chase Player if no nearest target found
  (Character|Crouch)
  (AI|Navigation|MovetoActor (AI|GetAIController self) (Game|GetPlayerCharacter 0) 2.0 true true true 0))

(event Custom|STATE%20ATTACKING%20Behaviour
  (bind _overlapped_actors (CallFunction|CheckOverlapwithAttackRange))
  ;[0.5117 0.7258 1] STATES
  ;;[1 0.4004 0.4803] Attacking STATE Logic
  (if (Utilities|Array|IsNotEmpty _overlapped_actors) :!label _label
    (Utilities|FlowControl|Delay (/ 1.0 (Variables|Default|GetAttack%20Speed)))
    (for _array_element _overlapped_actors
      (CallFunction|Attack(TargetonAttackRange) 0 _array_element) ; This can ve overridden easily by child actor
    )
    (goto _label)
    (else
      (CallFunction|SetSTATEandAnimation "NewEnumerator1")
      (CallFunction|ResetAttacking"DoOnce"AfterNoEnemyNearby))))

(event Custom|STATE%20DEATH%20Behaviour
  ;[0.5117 0.7258 1] STATES
)

(event EventBeginPlay
  ;[0.2622 1 0.2689] Default STATE and change to SEARCHING
  (CallFunction|SetSTATEandAnimation "NewEnumerator0")
  (Utilities|FlowControl|Delay (* (Math|Float|MakeLiteralFloat 5.0) (Math|Random|RandomFloat)))
  (CallFunction|SetSTATEandAnimation "NewEnumerator4"))

(event EventTick
  (params (DeltaSeconds :type Float%20%28single-precision%29))
  ;[1 0.8623 0.3364] STATE Handler from Event Tick
  (CallFunction|STATEBehaviour))

(event EventDies
  ;[1 0.4786 0.4686] Override the Event Dies so that it is handled by the function.
  (CallFunction|SetSTATEandAnimation "NewEnumerator3"))

(fn ConstructionScript)

(fn PlayAnimationbySTATE
  (params (Current%20STATE :type ENUM_ENEMY_STATE%20Enum :default "NewEnumerator0"))
  ;[1 1 1] Function should be overidden by child.
)

(fn SetSTATEandAnimation
  (params (New%20STATE :type ENUM_ENEMY_STATE%20Enum :default "NewEnumerator0"))
  (bind _output_get (Variables|Default|SetSTATE New%20STATE))
  (CallFunction|PlayAnimationbySTATE _output_get)
  ;[1 1 1] Only when changing the STATE to DEATH
  (if (Utilities|Enum|Equal(Enum) (Variables|Default|GetSTATE) "NewEnumerator3")
    (Utilities|FlowControl|DoOnce false
      (:Completed
        (Actor|SetLifeSpan 0.5)))))

(fn Attack(TargetonAttackRange)
  (params (Overlapped%20Component :type Primitive%20Component%20Object%20Reference) (Other%20Actor :type Actor%20Object%20Reference) (Other%20Component :type Primitive%20Component%20Object%20Reference))
  (bind _damage (Variables|Default|GetDamage))
  ;[1 1 1] This should be overridden by Child Actor (This is the default melee attack)
  (Game|Damage|ApplyDamage Other%20Actor _damage 0 self)
  ;[1 1 1] DEBUG: For printing who damages who
  (Development|PrintString (Utilities|String|Append (Utilities|GetDisplayName self) (Utilities|String|MakeLiteralString " (using Melee) damaged : ") (Utilities|GetDisplayName Other%20Actor) (Utilities|String|MakeLiteralString " by ") (Utilities|String|ToString(Float) _damage))))

(fn CheckOverlapwithAttackRange
  (bind _attack_range (Variables|Default|GetAttack%20Range))
  (Utilities|Set|AddItems (LocalVariables|GetBP_Turrets%20Set) (Collision|GetOverlappingActors _attack_range "/Game/Characters/Turrets/BP_Turrets.BP_Turrets_C" :!class /Script/Engine.PrimitiveComponent))
  (Utilities|Set|AddItems (LocalVariables|GetBP_ControllableCharacter%20Set) (Collision|GetOverlappingActors _attack_range "/Game/Characters/BP_ControllableCharacter.BP_ControllableCharacter_C" :!class /Script/Engine.PrimitiveComponent))
  (bind _result (Utilities|Set|Union (LocalVariables|GetBP_ControllableCharacter%20Set) (LocalVariables|GetBP_Turrets%20Set)))
  (bind _result_2 (Utilities|Set|ToArray _result))
  (return _result_2))