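; Speaker enemy character that damages player-controllable characters on sight, with its own starting health.
; When PawnSensing spots a BP_ControllableCharacter, Fire switches state and animation, disables movement and applies damage directly, without a projectile.
; Tick calls UpdateState, whose Delay restores the other state and NavWalking on a repeating few-second cycle, independent of when Fire last ran.
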(event OnSeePawn(PawnSensing)
  (params (Pawn :type Pawn%20Object%20Reference))
  (bind _asbp_controllable_character (Utilities|Casting|CastToBP_ControllableCharacter Pawn))
  (CallFunction|Fire _asbp_controllable_character))

(event Custom|Fire
  (params (Pawn :type Pawn%20Object%20Reference))
  (CallFunction|SetSTATEandAnimation "NewEnumerator2")
  (Pawn|Components|CharacterMovement|SetMovementMode (Variables|Character|GetCharacterMovement) "MOVE_None" 0)
  (Game|Damage|ApplyDamage Pawn (Variables|Default|GetDamage) 0 self))

(event Custom|Update%20State
  (Utilities|FlowControl|Delay 3.0)
  (CallFunction|SetSTATEandAnimation "NewEnumerator1")
  (Pawn|Components|CharacterMovement|SetMovementMode (Variables|Character|GetCharacterMovement) "MOVE_NavWalking" 0))

(event EventBeginPlay
  (|CallParentFunction)
  (Variables|Default|SetHealth 2e+02) ; Setting Default Health
)

(event Collision|EventActorBeginOverlap
  (params (OtherActor :type Actor%20Object%20Reference))
  (|CallParentFunction OtherActor) ; This node is disabled and will not be called.\nDrag off pins to build functionality.
)

(event EventTick
  (params (DeltaSeconds :type Float%20%28single-precision%29))
  (|CallParentFunction DeltaSeconds)
  (CallFunction|UpdateState))

(fn ConstructionScript
  (|CallParentFunction))