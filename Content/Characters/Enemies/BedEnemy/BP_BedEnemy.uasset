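; Bed enemy that attacks by throwing homing pillows, built on an inherited state-driven enemy.
; Its attacking state waits on attack speed, plays an animation, then spawns a BP_Pillow homing on the first actor in attack range.
; With nothing in range, it switches state and resets the attack gate.
; An empty override disables the inherited attack-range hit, leaving the pillow as its attack.
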(event EventBeginPlay
  (|CallParentFunction) ; This node is disabled and will not be called.\nDrag off pins to build functionality.
)

(event Collision|EventActorBeginOverlap
  (params (OtherActor :type Actor%20Object%20Reference))
  (|CallParentFunction OtherActor) ; This node is disabled and will not be called.\nDrag off pins to build functionality.
)

(event EventTick
  (params (DeltaSeconds :type Float%20%28single-precision%29))
  (|CallParentFunction DeltaSeconds) ; This node is disabled and will not be called.\nDrag off pins to build functionality.
)

(event EventSTATEATTACKINGBehaviour
  (bind _overlapped_actors (CallFunction|CheckOverlapwithAttackRange))
  (if (Utilities|Array|IsNotEmpty _overlapped_actors)
    (Utilities|FlowControl|Delay (/ 1.0 (Variables|Default|GetAttack%20Speed)))
    (Components|Animation|PlayAnimation (Variables|Character|GetMesh) "/Game/Characters/Enemies/BedEnemy/ranjang_gila_Anim.ranjang_gila_Anim" false)
    (Utilities|FlowControl|Delay 0.3)
    (bind _returnvalue (Game|SpawnActorfromClass "/Game/Characters/Enemies/BedEnemy/BP_Pillow.BP_Pillow_C" (Transformation|GetWorldTransform (Variables|Default|GetPillow%20Direction)) "AlwaysSpawn" "MultiplyWithRoot" 0 0))
    (Variables|/Script/Engine.ProjectileMovementComponent|SetHomingTargetComponent (Variables|/Game/Characters/Enemies/BedEnemy/BP_Pillow.BP_Pillow_C|GetProjectileMovement _returnvalue) (Variables|/Script/Engine.Actor|GetRootComponent (Utilities|Array|Get(acopy) _overlapped_actors)))
    (else
      (CallFunction|SetSTATEandAnimation "NewEnumerator1")
      (CallFunction|ResetAttacking"DoOnce"AfterNoEnemyNearby))))

(fn ConstructionScript
  (|CallParentFunction))

(fn Attack(TargetonAttackRange)
  (params (Overlapped%20Component :type Primitive%20Component%20Object%20Reference) (Other%20Actor :type Actor%20Object%20Reference) (Other%20Component :type Primitive%20Component%20Object%20Reference))
  ;[1 1 1] Override so that enemy doesn't attack with Attack Range
)