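; BP_Character is a character Blueprint that gives an actor basic health, damage and death handling.
; AnyDamage plays a hit sound, then either subtracts damage from Health and prints the result for debugging, or calls Dies when health would reach zero or below.
; Dies plays a sound and destroys the actor.
; Both sounds play at the world origin rather than at the character's location.
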(event EventBeginPlay)

(event Collision|EventActorBeginOverlap
  (params (OtherActor :type Actor%20Object%20Reference)))

(event EventTick
  (params (DeltaSeconds :type Float%20%28single-precision%29)))

(event EventDies
  (Audio|PlaySoundatLocation "/Game/SoundEffects/footstep07.footstep07" "0, 0, 0" "0, 0, 0" 1.0 1.0 0.0 0 0 0 0)
  (Actor|DestroyActor))

(event EventGotHitSoundEffect
  (Audio|PlaySoundatLocation "/Game/SoundEffects/handleCoins.handleCoins" "0, 0, 0" "0, 0, 0" 1.0 1.0 0.0 0 0 0 0))

(event Game|Damage|EventAnyDamage
  (params (Damage :type Float%20%28single-precision%29) (DamageType :type Damage%20Type%20Object%20Reference) (InstigatedBy :type Controller%20Object%20Reference) (DamageCauser :type Actor%20Object%20Reference))
  ;[1 0.2033 0.3535] Character Taking Damage Logic
  (CallFunction|GotHitSoundEffect)
  (if (> (- (Variables|Default|GetHealth) Damage) 0.0)
    (bind _output_get (Variables|Default|SetHealth (- (Variables|Default|GetHealth) Damage)))
    ;;[1 1 1] Print Health (Debug)
    (Development|PrintString (Utilities|String|Append (Utilities|String|Append (Utilities|GetDisplayName self) (Utilities|String|MakeLiteralString " Health : ")) (Utilities|String|ToString(Float) _output_get)))
    (else
      (CallFunction|Dies) ; Target Dies
    )))

(fn ConstructionScript)