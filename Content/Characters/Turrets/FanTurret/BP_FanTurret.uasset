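; BP_FanTurret is a turret that pushes enemies with bursts of force.
; One second after BeginPlay, it starts the looping fan animation unless TurretState is the first enum value.
; Outside that state, Tick calls FireSlow through a DoOnce that a two-second Delay resets, throttling the bursts.
; Each burst applies a velocity-change impulse along Direction's forward vector to every BP_Enemy overlapping ForceArea, scaled by ForcePower.
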(event Custom|Fire%20Slow
  (Utilities|FlowControl|DoOnce false
    (:Completed
      (for _array_element (Collision|GetOverlappingActors (Variables|Default|GetForce%20Area) 0 :!class /Script/Engine.PrimitiveComponent)
        (bind _asbp_enemy (Utilities|Casting|CastToBP_Enemy _array_element))
        (Physics|AddImpulse (Variables|/Script/Engine.Character|GetCharacterMovement _asbp_enemy) (* (Math|Vector|GetForwardVector (Variables|Default|GetDirection)) (Math|Float|MakeLiteralFloat (Variables|Default|GetForce%20Power))) true)
        (Development|PrintString "added impulse")))))

(event EventBeginPlay
  (|CallParentFunction)
  (Utilities|FlowControl|Delay 1.0)
  (if (not (Utilities|Enum|Equal(Enum) (Variables|Default|GetTurretState) "NewEnumerator0"))
    (Components|Animation|PlayAnimation (Variables|Default|GetFan%20Fan) "/Game/Characters/Turrets/FanTurret/fan_fan_Anim.fan_fan_Anim" true)))

(event Collision|EventActorBeginOverlap
  (params (OtherActor :type Actor%20Object%20Reference))
  (|CallParentFunction OtherActor) ; This node is disabled and will not be called.\nDrag off pins to build functionality.
)

(event EventTick
  (params (DeltaSeconds :type Float%20%28single-precision%29))
  (|CallParentFunction DeltaSeconds)
  (if (not (Utilities|Enum|Equal(Enum) (Variables|Default|GetTurretState) "NewEnumerator0"))
    (CallFunction|FireSlow)
    (Utilities|FlowControl|Delay 2.0)
    (Utilities|FlowControl|DoOnce false) ; enters at Reset
  ))

(fn ConstructionScript
  (|CallParentFunction))