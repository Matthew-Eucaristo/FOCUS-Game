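; Scissor turret that deals area damage to overlapping enemies when tagged turret targets enter or leave its attack range, unless its state blocks it.
; An attack plays ruler and scissor animations with a sword sound, then damages every BP_Enemy in range.
; DoOnce gates throttle attacks, reset after a delay, and the brief fire-circle particle burst, reset as damage is applied.
; Attacks are driven only by overlap events, with no timer loop or Tick.
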(event OnComponentBeginOverlap(AttackRange)
  (params (OverlappedComponent :type Primitive%20Component%20Object%20Reference) (OtherActor :type Actor%20Object%20Reference) (OtherComp :type Primitive%20Component%20Object%20Reference) (OtherBodyIndex :type Integer) (bFromSweep :type Boolean) (SweepResult :type Hit%20Result%20Structure%20%28by%20ref%29))
  (bind _p_aoe_fire_circleattack (Variables|Default|GetP_AOE_Fire_CircleAttack))
  (if (and (Actor|ActorHasTag OtherActor "Turret Targets") (Utilities|Enum|NotEqual(Enum) (Variables|Default|GetTurretState) "NewEnumerator0"))
    (CallFunction|Attack)
    (Utilities|FlowControl|Delay 2.0)
    (Utilities|FlowControl|DoOnce false) ; enters at Reset
  ))

(event OnComponentEndOverlap(AttackRange)
  (params (OverlappedComponent :type Primitive%20Component%20Object%20Reference) (OtherActor :type Actor%20Object%20Reference) (OtherComp :type Primitive%20Component%20Object%20Reference) (OtherBodyIndex :type Integer))
  (bind _p_aoe_fire_circleattack (Variables|Default|GetP_AOE_Fire_CircleAttack))
  (if (and (Actor|ActorHasTag OtherActor "Turret Targets") (Utilities|Enum|NotEqual(Enum) (Variables|Default|GetTurretState) "NewEnumerator0"))
    (CallFunction|Attack)
    (Utilities|FlowControl|Delay 2.0)
    (Utilities|FlowControl|DoOnce false) ; enters at Reset
  ))

(event Custom|Attack
  (bind _p_aoe_fire_circleattack (Variables|Default|GetP_AOE_Fire_CircleAttack))
  (CallFunction|Activate/DeactivateParticleSystem)
  (Utilities|FlowControl|DoOnce false
    (:Completed
      (Components|Animation|PlayAnimation (Variables|Default|GetRuler) "/Game/Characters/Turrets/ScissorTurret/ruler_Anim_Cube_CubeAction.ruler_Anim_Cube_CubeAction" false)
      (Audio|PlaySoundatLocation "/Game/Characters/Turrets/ScissorTurret/Assets/SFX/sword-sound-2-36274.sword-sound-2-36274" (Transformation|GetWorldLocation (Variables|Default|GetDefaultSceneRoot)) "0, 0, 0" 1.0 1.0 0.0 0 0 0 0)
      (Components|Animation|PlayAnimation (Variables|Default|GetScissor) "/Game/Characters/Turrets/ScissorTurret/scissor_Anim_group105737810_CubeAction.scissor_Anim_group105737810_CubeAction" false)
      (for _array_element (Collision|GetOverlappingActors (Variables|Default|GetAttack%20Range) "/Game/Characters/Enemies/BP_Enemy.BP_Enemy_C" :!class /Script/Engine.PrimitiveComponent)
        (Game|Damage|ApplyDamage _array_element (Variables|Default|GetDamage) 0 0)
        (Utilities|FlowControl|DoOnce false) ; enters at Reset
      ))))

(event Custom|Activate/Deactivate%20Particle%20System
  (bind _p_aoe_fire_circleattack (Variables|Default|GetP_AOE_Fire_CircleAttack))
  (Utilities|FlowControl|DoOnce false
    (:Completed
      (Components|Activation|Activate _p_aoe_fire_circleattack false)
      (Utilities|FlowControl|Delay 1.0)
      (Components|Activation|Deactivate _p_aoe_fire_circleattack))))

(event EventBeginPlay
  (|CallParentFunction) ; This node is disabled and will not be called.\nDrag off pins to build functionality.
)

(event Collision|EventActorBeginOverlap
  (params (OtherActor :type Actor%20Object%20Reference))
  (|CallParentFunction OtherActor) ; This node is disabled and will not be called.\nDrag off pins to build functionality.
)

(event EventTick
  (params (DeltaSeconds :type Float%20%28single-precision%29))
  (|CallParentFunction DeltaSeconds) ; This node is disabled and will not be called.\nDrag off pins to build functionality.
)

(fn ConstructionScript
  (|CallParentFunction))