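; BP_MagicBook is a magic book turret that repeatedly fires BP_MagicWord projectiles.
; Tick runs into a two-second Delay, which works as a repeating fire timer without any target checks.
; Each shot always spawns at the SpawnArrow's location, taking no rotation from it, then gets its ProjectileMovement velocity set along the projectile's local Z axis.
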(event EventBeginPlay
  (|CallParentFunction) ; This node is disabled and will not be called.\nDrag off pins to build functionality.
)

(event Collision|EventActorBeginOverlap
  (params (OtherActor :type Actor%20Object%20Reference))
  (|CallParentFunction OtherActor) ; This node is disabled and will not be called.\nDrag off pins to build functionality.
)

(event EventTick
  (params (DeltaSeconds :type Float%20%28single-precision%29))
  (|CallParentFunction DeltaSeconds)
  (Utilities|FlowControl|Delay 2.0)
  (bind _returnvalue (Game|SpawnActorfromClass "/Game/Characters/Turrets/MagicBook/BP_MagicWord.BP_MagicWord_C" (Math|Transform|MakeTransform (Transformation|GetWorldLocation (Variables|Default|GetSpawn%20Arrow)) "0, 0, 0" "1.000000,1.000000,1.000000") "AlwaysSpawn" "MultiplyWithRoot" 0 0))
  (Utilities|IsValid _returnvalue
    (:Is%20Valid
      (Game|Components|ProjectileMovement|SetVelocityinLocalSpace (Variables|/Game/Characters/Turrets/MagicBook/BP_MagicWord.BP_MagicWord_C|GetProjectileMovement _returnvalue) "0.000000,0.000000,1500.000000"))))

(fn ConstructionScript
  (|CallParentFunction))