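; BP_MagicWord is a magic word projectile for the Magic Book turret that orbits its spawn point, then homes in on enemies.
; AdditionalTime picks its Niagara element effect, offsets its orbit phase and staggers its launch.
; A repeating LockOn feeds the box component of the nearest "Turret Targets" actor to ProjectileMovement, or moves toward TargetLastLocation without one.
; Hitting a BP_Enemy launches and damages it, then destroys the word.
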(event OnComponentBeginOverlap(Collision)
  (params (OverlappedComponent :type Primitive%20Component%20Object%20Reference) (OtherActor :type Actor%20Object%20Reference) (OtherComp :type Primitive%20Component%20Object%20Reference) (OtherBodyIndex :type Integer) (bFromSweep :type Boolean) (SweepResult :type Hit%20Result%20Structure%20%28by%20ref%29)))

(event Custom|Lock%20On
  (bind _projectilemovement (Variables|Default|GetProjectileMovement))
  (bind _homing_target (CallFunction|FindHomingTarget))
  (if (Utilities|IsValid _homing_target)
    (Variables|/Script/Engine.ProjectileMovementComponent|SetHomingTargetComponent _projectilemovement _homing_target)
    (Utilities|FlowControl|Delay 0.2)
    (Variables|/Script/Engine.ProjectileMovementComponent|SetbIsHomingProjectile _projectilemovement true)
    (else
      (Components|MoveComponentTo 0 (Variables|Default|GetTargetLastLocation) "0, 0, 0" false false 0.2 false))))

(event EventBeginPlay
  (bind _staticmesh (Variables|Default|GetStaticMesh))
  (Variables|Default|SetNumber (Math|Float|Truncate (/ (Variables|Default|GetadditionalTime) 1.3)))
  (Variables|Default|SetTime (+ (Variables|Default|GetTime) (Variables|Default|GetadditionalTime)))
  (switch int (Variables|Default|GetNumber)
    (:Default
      (Niagara|SpawnSystemAttached "/Game/Characters/Turrets/MagicBook/PIElement.PIElement" _staticmesh "None" "0, 0, 0" "0, 0, 0" "KeepRelativeOffset" false :!label _label))
    (:1
      (goto _label))
    (:2
      (Niagara|SpawnSystemAttached "/Game/Characters/Turrets/MagicBook/AIElement.AIElement" _staticmesh "None" "0, 0, 0" "0, 0, 0" "KeepRelativeOffset" false))
    (:3
      (Niagara|SpawnSystemAttached "/Game/Characters/Turrets/MagicBook/AtomElement.AtomElement" _staticmesh "None" "0, 0, 0" "0, 0, 0" "KeepRelativeOffset" false))
    (:4
      (Niagara|SpawnSystemAttached "/Game/Characters/Turrets/MagicBook/PEElement.PEElement" _staticmesh "None" "0, 0, 0" "0, 0, 0" "KeepRelativeOffset" false))
    (:5
      (Niagara|SpawnSystemAttached "/Game/Characters/Turrets/MagicBook/SocialElement.SocialElement" _staticmesh "None" "0, 0, 0" "0, 0, 0" "KeepRelativeOffset" false)))
  (Variables|Default|SetOriginal%20Position (Transformation|GetActorLocation))
  (Utilities|FlowControl|Delay (+ (Variables|Default|GetPrepTime) (/ (Variables|Default|GetadditionalTime) 2.0)))
  (CallFunction|Lockon :!label _label_2)
  (Utilities|FlowControl|Delay 0.1)
  (goto _label_2))

(event Collision|EventHit
  (params (MyComp :type Primitive%20Component%20Object%20Reference) (Other :type Actor%20Object%20Reference) (OtherComp :type Primitive%20Component%20Object%20Reference) (bSelfMoved :type Boolean) (HitLocation :type Vector :default "0, 0, 0") (HitNormal :type Vector :default "0, 0, 0") (NormalImpulse :type Vector :default "0, 0, 0") (Hit :type Hit%20Result%20Structure%20%28by%20ref%29))
  (bind _asbp_enemy (Utilities|Casting|CastToBP_Enemy Other)
    (:then
      (Utilities|FlowControl|DoOnce false
        (:Completed
          (Variables|Default|SetTargetLastLocation (Transformation|GetActorLocation Other))
          (Character|LaunchCharacter _asbp_enemy (Transformation|GetVelocity) false false)
          (Game|Damage|ApplyDamage _asbp_enemy 5e+01 0 0)
          (Actor|DestroyActor))))
    (:CastFailed
      (if (not (Actor|ActorHasTag Other "Homing"))
        (Actor|DestroyActor)))))

(event EventTick
  (params (DeltaSeconds :type Float%20%28single-precision%29))
  (bind _original_position (Variables|Default|GetOriginal%20Position))
  (if (not (Variables|/Script/Engine.ProjectileMovementComponent|GetbIsHomingProjectile (Variables|Default|GetProjectileMovement)))
    (Variables|Default|SetTime (+ DeltaSeconds (Variables|Default|GetTime)))
    (bind _output_get (Variables|Default|SetCirclePosition (Math|Vector|MakeVector (+ (* (Math|Trig|Cos(Radians) (Variables|Default|GetTime)) -1.5e+02) (.x _original_position)) (+ (* (Math|Trig|Sin(Radians) (Variables|Default|GetTime)) -1.5e+02) (.y _original_position)) (.z _original_position))))
    (Transformation|SetActorLocation _output_get false false)))

(fn ConstructionScript)

(fn FindHomingTarget
  (bind _outactors (Actor|GetAllActorsOfClasswithTag "/Script/Engine.Actor" "Turret Targets"))
  ;[1 1 1] Get Closest Target
  (for _array_element _outactors
    (if (Actor|ActorHasTag _array_element "Turret Targets")
      (if (< (Math|Vector|VectorLength (- (Transformation|GetActorLocation _array_element) (Transformation|GetActorLocation))) (Variables|Default|GetClosest%20Distance))
        (Variables|Default|SetClosest%20Distance (Math|Vector|VectorLength (- (Transformation|GetActorLocation _array_element) (Transformation|GetActorLocation))))
        (Variables|Default|SetHoming%20Target _array_element))))
  (if (Utilities|IsValid (Variables|Default|GetHoming%20Target))
    (return (Actor|GetComponentbyClass (Variables|Default|GetHoming%20Target) "/Script/Engine.BoxComponent"))))