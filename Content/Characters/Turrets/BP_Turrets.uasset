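; Turret actor that handles its own health and validates where it can be placed.
; TakeDamage plays a hit sound and lowers Health, calling Dies to destroy the actor when the damage would deplete it.
; CheckSpawn sets CanSpawn by whether the placement collision is free of overlaps, tinting the static meshes under ParentMesh with a green or red overlay material as placement feedback.
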(event EventBeginPlay)

(event Collision|EventActorBeginOverlap
  (params (OtherActor :type Actor%20Object%20Reference)))

(event EventTick
  (params (DeltaSeconds :type Float%20%28single-precision%29)))

(event EventTakeDamage
  (params (Damage :type Float%20%28double-precision%29))
  (CallFunction|GotHitSoundEffect)
  (if (> (- (Variables|Default|GetHealth) Damage) 0.0)
    (Variables|Default|SetHealth (- (Variables|Default|GetHealth) Damage))
    (else
      (CallFunction|Dies) ; Target Dies
    )))

(event EventDies
  (Actor|DestroyActor))

(fn ConstructionScript)

(fn CheckSpawn
  (bind _parent_mesh (Variables|Default|GetParent%20Mesh))
  (bind _children (Components|GetChildrenComponents _parent_mesh true))
  (if (Utilities|Array|IsEmpty (Class|PrimitiveComponent|GetOverlappingComponents (Variables|Default|GetTurret%20Placement%20Collision)))
    (for _array_element _children
      (bind _asstatic_mesh_component (Utilities|Casting|CastToStaticMeshComponent _array_element))
      (Rendering|Material|SetOverlayMaterial _asstatic_mesh_component "/Game/Characters/Turrets/TurretMaterials/InvisibleGreen.InvisibleGreen" :!class /Script/Engine.MeshComponent))
    (Variables|Default|SetbCanSpawn true)
    (else
      (for _array_element_2 _children
        (bind _asstatic_mesh_component_2 (Utilities|Casting|CastToStaticMeshComponent _array_element_2))
        (Rendering|Material|SetOverlayMaterial _asstatic_mesh_component_2 "/Game/Characters/Turrets/TurretMaterials/InvisibleRed.InvisibleRed" :!class /Script/Engine.MeshComponent))
      (Variables|Default|SetbCanSpawn false))))