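; BP_Grenade is a grenade item actor that explodes on a timer once thrown.
; On BeginPlay, if HasThrown is set, it waits a short fuse, then applies radial damage with falloff that ignores the player character.
; It plays an explosion sound and particle effect, hides the Grenade component, and destroys itself after a further delay.
; Instances without HasThrown set never start the fuse.
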(event EventBeginPlay
  (bind _returnvalue (Transformation|GetActorLocation))
  (|CallParentFunction)
  (if (Variables|Default|GetbHasThrown)
    (Utilities|FlowControl|Delay 2.0)
    (Class|GameplayStatics|ApplyRadialDamagewithFalloff 2e+02 5e+01 (Transformation|GetActorLocation) 3e+02 5e+02 1.0 0 (Utilities|Array|MakeArray (Game|GetPlayerCharacter 0)) self 0 "ECC_Visibility")
    (Audio|PlaySoundatLocation "/Game/SoundEffects/Grenade/grenade_Cue.grenade_Cue" _returnvalue "0, 0, 0" 1.0 1.0 0.0 0 0 0 0)
    (Effects|SpawnEmitteratLocation "/Game/StarterContent/Particles/P_Explosion.P_Explosion" _returnvalue "0, 0, 0" "3.000000,3.000000,3.000000")
    (Development|SetHiddeninGame (Variables|Default|GetGrenade) true false)
    (Utilities|FlowControl|Delay 2.0)
    (Actor|DestroyActor)))

(event Collision|EventActorBeginOverlap
  (params (OtherActor :type Actor%20Object%20Reference))
  (|CallParentFunction OtherActor) ; This node is disabled and will not be called.\nDrag off pins to build functionality.
)

(event EventTick
  (params (DeltaSeconds :type Float%20%28single-precision%29))
  (|CallParentFunction DeltaSeconds))

(event Collision|EventHit
  (params (MyComp :type Primitive%20Component%20Object%20Reference) (Other :type Actor%20Object%20Reference) (OtherComp :type Primitive%20Component%20Object%20Reference) (bSelfMoved :type Boolean) (HitLocation :type Vector :default "0, 0, 0") (HitNormal :type Vector :default "0, 0, 0") (NormalImpulse :type Vector :default "0, 0, 0") (Hit :type Hit%20Result%20Structure%20%28by%20ref%29)))

(fn ConstructionScript
  (|CallParentFunction))