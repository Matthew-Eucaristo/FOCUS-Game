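; BP_Pets is a pet character that switches behaviour state based on its distance to the player.
; Each tick it writes its PetSTATE enum to the AI controller's blackboard, then checks player proximity within a fixed radius.
; Leaving the radius changes state immediately, while being inside applies the other state after a short delay.
; A Bark function plays a sound cue at the pet's location.
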(event Custom|Check%20if%20the%20player%20is%20too%20far
  (if (CallFunction|IsClosetoPlayer 6e+02)
    (Utilities|FlowControl|Delay 2.0)
    (Variables|Default|SetPet%20STATE "NewEnumerator0")
    (else
      (Variables|Default|SetPet%20STATE "NewEnumerator1"))))

(event EventBeginPlay)

(event Collision|EventActorBeginOverlap
  (params (OtherActor :type Actor%20Object%20Reference)))

(event EventTick
  (params (DeltaSeconds :type Float%20%28single-precision%29))
  ;[1 1 1] Set the value in the blackboard to the value of the STATE
  (AI|Components|Blackboard|SetValueasEnum (AI|GetBlackboard (AI|GetAIController self)) (Utilities|Name|MakeLiteralName "PET STATE") (Variables|Default|GetPet%20STATE))
  (CallFunction|CheckifthePlayerIsTooFar))

(fn ConstructionScript)

(fn IsClosetoPlayer
  (params (Accepted%20Distance :type Float%20%28double-precision%29))
  (return (<= (Math|Vector|Distance(Vector) (Transformation|GetWorldLocation (Variables|/Script/Engine.Character|GetCapsuleComponent (Game|GetPlayerCharacter 0))) (Transformation|GetWorldLocation (Variables|Collision|GetCapsuleComponent))) Accepted%20Distance)))

(fn Bark
  (Audio|PlaySoundatLocation "/Game/Pets/ShibaInu/Audio/Cue_Bark.Cue_Bark" (Transformation|GetWorldLocation (Variables|Collision|GetCapsuleComponent)) "0, 0, 0" 1.0 1.0 0.0 0 0 0 0))