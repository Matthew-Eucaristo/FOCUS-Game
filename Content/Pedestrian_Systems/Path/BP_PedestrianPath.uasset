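; BP_PedestrianPath is a spline-based path actor that populates a pedestrian route at runtime.
; On BeginPlay it walks the PathForPedestrian spline in two passes, spawning BP_Spawner actors at a fixed interval, then BP_WayPoint actors every DistanceBetweenWaypoints units.
; Each pass starts at the spline's beginning and loops in world space until the distance reaches the spline length.
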(event Custom|Place%20Pedestrian%20WayPoints
  ;[0.1661 0.3253 1] Where to Place Pedestrian WayPoints
  (Variables|Default|SetSpline%20Distance 0.0)
  (Game|SpawnActorfromClass "/Game/Pedestrian_Systems/Waypoint/BP_WayPoint.BP_WayPoint_C" (Math|Transform|MakeTransform (Spline|GetLocationatDistanceAlongSpline (Variables|Default|GetPathForPedestrian) (Variables|Default|GetSpline%20Distance) "World") "0, 0, 0" "1.000000,1.000000,1.000000") "Undefined" "OverrideRootScale" 0 0 :!label _label)
  (bind _output_get (Variables|Default|SetSpline%20Distance (+ (Variables|Default|GetSpline%20Distance) (Variables|Default|GetDistance%20Between%20Waypoints))))
  (if (< _output_get (Spline|GetSplineLength (Variables|Default|GetPathForPedestrian)))
    (goto _label)))

(event Custom|Place%20Pedestrian%20Spawners
  ;[0.1978 0.2996 1] Where To Place Pedestrian Spawners
  (Variables|Default|SetSpline%20Distance 0.0)
  (Game|SpawnActorfromClass "/Game/Pedestrian_Systems/Spawner/BP_Spawner.BP_Spawner_C" (Math|Transform|MakeTransform (Spline|GetLocationatDistanceAlongSpline (Variables|Default|GetPathForPedestrian) (Variables|Default|GetSpline%20Distance) "World") "0, 0, 0" "1.000000,1.000000,1.000000") "Undefined" "OverrideRootScale" 0 0 :!label _label)
  (bind _output_get (Variables|Default|SetSpline%20Distance (+ (Variables|Default|GetSpline%20Distance) 6e+02)))
  (if (< _output_get (Spline|GetSplineLength (Variables|Default|GetPathForPedestrian)))
    (goto _label)))

(event EventBeginPlay
  ;[1 1 1] Place spawners and waypoints on begin play
  (CallFunction|PlacePedestrianSpawners)
  (CallFunction|PlacePedestrianWayPoints))

(fn ConstructionScript)