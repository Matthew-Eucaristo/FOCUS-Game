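; Demo pedestrian character that randomizes its appearance on spawn and supports behavior switching.
; BeginPlay picks a random body mesh and material, loops a walk animation in single-node mode, and starts a timeline as a custom tick.
; That tick calls the plugin's PedestrianDestroyer component to cull by distance from the player.
; Events toggle the AI blackboard's wandering key, or halt movement for a montage and later restore walking.
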(event Custom|Destroy%20By%20distance
  ;[1 1 1] Destroy By Distance From Player
  (Class|PedestrianDestroyer|DestroybyDistance (Variables|Default|GetPedestrianDestroyer) (Variables|Default|GetDistance%20To%20Destroy)) ; Part of the "Pedestrian Destroyer" component from plugin
)

(event Custom|ToggleBehaviorType
  (bind _returnvalue (Utilities|Name|MakeLiteralName "ActivateWandering"))
  (bind _self self)
  (bind _returnvalue_2 (AI|GetAIController _self))
  (bind _returnvalue_3 (AI|GetBlackboard _returnvalue_2))
  ;[1 1 1] Toggle blackboard key value for switching behavior types(Delegate from Player) *Can delete only for demo purposes
  (Utilities|FlowControl|FlipFlop
    (:A
      (AI|Components|Blackboard|SetValueasBool _returnvalue_3 _returnvalue true))
    (:B
      (AI|Components|Blackboard|SetValueasBool _returnvalue_3 _returnvalue false))))

(event EventBeginPlay
  (bind _returnvalue (Math|Random|RandomInteger 4))
  (bind _custommesh (Variables|Default|GetCustomMesh))
  (bind _custommesh_2 (Variables|Default|GetCustomMesh))
  (Components|SkeletalMesh|SetSkeletalMeshAsset _custommesh_2 (Utilities|Select :Index _returnvalue :Option%200 "/Game/KenneysCharacters/Models/characterLargeMale.characterLargeMale" :Option%201 "/Game/KenneysCharacters/Models/characterLargeFemale.characterLargeFemale" :Option%202 "/Game/KenneysCharacters/Models/characterMedium.characterMedium" :Option%203 "/Game/KenneysCharacters/Models/characterSmall.characterSmall"))
  (Rendering|Material|SetMaterial _custommesh_2 0 (Utilities|Select :Index (Math|Random|RandomInteger 20) :Option%200 "/Game/KenneysCharacters/Skins/astroFemaleA_Mat.astroFemaleA_Mat" :Option%201 "/Game/KenneysCharacters/Skins/astroFemaleB_Mat.astroFemaleB_Mat" :Option%202 "/Game/KenneysCharacters/Skins/astroMaleA_Mat.astroMaleA_Mat" :Option%203 "/Game/KenneysCharacters/Skins/athleteFemaleBlue_Mat.athleteFemaleBlue_Mat" :Option%204 "/Game/KenneysCharacters/Skins/athleteFemaleGreen_Mat.athleteFemaleGreen_Mat" :Option%205 "/Game/KenneysCharacters/Skins/athleteFemaleRed_Mat.athleteFemaleRed_Mat" :Option%206 "/Game/KenneysCharacters/Skins/athleteMaleBlue_Mat.athleteMaleBlue_Mat" :Option%207 "/Game/KenneysCharacters/Skins/athleteMaleGreen_Mat.athleteMaleGreen_Mat" :Option%208 "/Game/KenneysCharacters/Skins/athleteMaleRed_Mat.athleteMaleRed_Mat" :Option%209 "/Game/KenneysCharacters/Skins/athleteMaleYellow_Mat.athleteMaleYellow_Mat" :Option%2010 "/Game/KenneysCharacters/Skins/businessMaleB_Mat.businessMaleB_Mat" :Option%2011 "/Game/KenneysCharacters/Skins/casualFemaleA_Mat.casualFemaleA_Mat" :Option%2012 "/Game/KenneysCharacters/Skins/casualMaleA_Mat.casualMaleA_Mat" :Option%2013 "/Game/KenneysCharacters/Skins/casualMaleB_Mat.casualMaleB_Mat" :Option%2014 "/Game/KenneysCharacters/Skins/cyborg_Mat.cyborg_Mat" :Option%2015 "/Game/KenneysCharacters/Skins/fantasyFemaleA_Mat.fantasyFemaleA_Mat" :Option%2016 "/Game/KenneysCharacters/Skins/racerBlueMale_Mat.racerBlueMale_Mat" :Option%2017 "/Game/KenneysCharacters/Skins/racerGreenFemale_Mat.racerGreenFemale_Mat" :Option%2018 "/Game/KenneysCharacters/Skins/survivorMaleA_Mat.survivorMaleA_Mat" :Option%2019 "/Game/KenneysCharacters/Skins/survivorMaleB_Mat.survivorMaleB_Mat"))
  (Components|Animation|SetAnimationMode _custommesh "AnimationSingleNode" true)
  (switch int _returnvalue
    (:0
      (Components|Animation|PlayAnimation _custommesh "/Game/KenneysCharacters/Animations/LargeMale/walk_Root_Walk.walk_Root_Walk" true)
      ;[1 1 1] Call the Destroy By Distance function on a looped timeline tick *Is Optional in your own project but reccommended for optimization
      (Timeline|CustomTick PlayFromStart
        (:Update
          (CallFunction|DestroybyDistance))))
    (:1
      (Components|Animation|PlayAnimation _custommesh "/Game/KenneysCharacters/Animations/LargeFemale/walk_Root_Walk.walk_Root_Walk" true)
      (Timeline|CustomTick PlayFromStart))
    (:2
      (Components|Animation|PlayAnimation _custommesh "/Game/KenneysCharacters/Animations/Medium/walk_Root_Walk.walk_Root_Walk" true)
      (Timeline|CustomTick PlayFromStart))
    (:3
      (Components|Animation|PlayAnimation _custommesh "/Game/KenneysCharacters/Animations/Small/walk_Root_Walk.walk_Root_Walk" true)
      (Timeline|CustomTick PlayFromStart))))

(event EventNPCAction1
  (Pawn|Components|CharacterMovement|DisableMovement (Variables|Character|GetCharacterMovement))
  (Animation|Montage|PlayMontage (Variables|Character|GetMesh) (Variables|Default|GetMontage%20to%20Play)))

(event EventNPCAction2
  (Pawn|Components|CharacterMovement|SetMovementMode (Variables|Character|GetCharacterMovement) "MOVE_Walking" 0)
  (Animation|StopAnimMontage (Variables|Default|GetMontage%20to%20Play)))

(fn ConstructionScript)